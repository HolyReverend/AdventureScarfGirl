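; BPC_HintKeyText is a hint text component that shows "Press" plus the key bound to its configured input action.
; One second after BeginPlay, it fetches key mappings from the first player controller and searches for the one matching IAAction.
; It sets the text using that key's long display name, then fires KeyTextObtained.
; With no matching action, it still sets text from the loop's leftover element.
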(event EventBeginPlay
  (Utilities|FlowControl|Delay 1.0)
  (CallFunction|ConfigureKeyDisplay))

(event EventTick
  (params (DeltaSeconds :type Float%20%28single-precision%29)))

(fn ConfigureKeyDisplay
  (bind _playercontrollkeys (Class|BPIPlayerControllerState|GetPlayerControllKeys(Message) (Game|GetPlayerController 0)))
  (bind _array_element (Utilities|Array|ForEachLoopwithBreak _playercontrollkeys :!label _label)
    (:LoopBody
      (if (== (.InputAction (Utilities|Struct|BreakST_PlayerControlKeys _array_element)) (Variables|KeyMapped|GetIA_Action))
        (goto _label Break)))
    (:Completed
      (Rendering|Components|TextRender|SetText (Utilities|Text|FormatText "Press {button}" (Class|KismetInputLibrary|KeyGetDisplayName (.Key (Utilities|Struct|BreakST_PlayerControlKeys _array_element)) true)))
      (Default|CallKeyTextObtained))))