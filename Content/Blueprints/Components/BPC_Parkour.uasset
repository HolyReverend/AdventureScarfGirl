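; Parkour component that probes for obstacles in front of its owner when the G debug key is pressed.
; A forward line trace finds a WorldStatic obstacle, then an upward trace from the impact point checks for clearance.
; If that is clear, a downward trace runs at a fixed distance ahead of the owner.
; All traces draw debug lines; the last result is unused and no movement is implemented.
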(event EventBeginPlay)

(event EventTick
  (params (DeltaSeconds :type Float%20%28single-precision%29)))

(event Input|KeyboardEvents|DebugKeyG
  (params (Key :type Key%20Structure :default "None") (ActionValue :type Input%20Action%20Value%20Structure))
  (bind _returnvalue (Components|GetOwner))
  (bind _returnvalue_2 (Components|GetOwner))
  (bind _returnvalue_3 (Transformation|GetActorLocation _returnvalue))
  (bind _returnvalue_4 (Transformation|GetActorForwardVector _returnvalue))
  (bind _returnvalue_5 (Transformation|GetActorLocation _returnvalue_2))
  (bind _returnvalue_6 (* _returnvalue_4 2e+02))
  (bind _returnvalue_7 (+ _returnvalue_3 _returnvalue_6))
  (:Pressed
    (bind (_outhit _returnvalue_8) (Collision|LineTraceForObjects _returnvalue_5 (+ _returnvalue_5 (* (Transformation|GetActorForwardVector _returnvalue_2) 5e+02)) (Utilities|Array|MakeArray "ObjectTypeQuery1") false 0 "ForDuration" true "(R=0.040928,G=0.000000,B=1.000000,A=1.000000)" "(R=1.000000,G=0.149448,B=0.000000,A=1.000000)"))
    (if _returnvalue_8
      (bind _returnvalue_9 (Collision|LineTraceForObjects (.ImpactPoint (Collision|BreakHitResult _outhit)) (+ (.ImpactPoint (Collision|BreakHitResult _outhit)) "0.000000,0.000000,150.000000") (Utilities|Array|MakeArray "ObjectTypeQuery1") false 0 "ForDuration" true "(R=0.000000,G=0.022305,B=1.000000,A=1.000000)" "(R=1.000000,G=0.169558,B=0.000000,A=1.000000)"))
      (if (not _returnvalue_9)
        (Collision|LineTraceForObjects (+ _returnvalue_7 "0.000000,0.000000,150.000000") _returnvalue_7 (Utilities|Array|MakeArray "ObjectTypeQuery1") false 0 "ForDuration" true "(R=0.000000,G=0.022305,B=1.000000,A=1.000000)" "(R=1.000000,G=0.169558,B=0.000000,A=1.000000)")))))