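; Character component that lets its owner attach to and push pushable actors, talking to the owner through message calls.
; BeginInteractPush picks the nearest attach point in range, validates space, floor and line of sight with traces, snaps the character there and attaches the object to it.
; Tick runs only while pushing, using box and line traces to switch move type when blocked or detach when obstructed.
; Debug status toggles trace drawing.
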(event EventBeginPlay
  (Components|Tick|SetComponentTickEnabled false))

(event EventTick
  (params (DeltaSeconds :type Float%20%28single-precision%29))
  (bind _returnvalue (Components|GetOwner))
  (switch Utilities|FlowControl|Switch|SwitchonE_PushableState (Pushing|CheckPushObstruction)
    (:NewEnumerator0
      (Class|BPICharacterState|SwitchCharacterMoveType(Message) _returnvalue "NewEnumerator2"))
    (:NewEnumerator1
      (Class|BPICharacterState|SwitchCharacterMoveType(Message) _returnvalue "NewEnumerator3"))
    (:NewEnumerator2
      (CallFunction|EndInteractPush (Variables|Default|GetCurrentActorPushing)))))

(fn StartPushing
  (Variables|Default|GetCurrentActorPushing
    (:then
      (bind _returnvalue (Transformation|AttachActorToActor (Variables|Default|GetCurrentActorPushing) (Components|GetOwner) "None" "KeepWorld" "KeepWorld" "KeepWorld" false))
      (if _returnvalue
        (Class|BPICharacterState|SendPushSpeedMult(Message) (Components|GetOwner) (Default|GetPushSpeedMult (Variables|Default|GetCurrentActorPushing)))
        (Class|BPICharacterState|SwitchCharacterMoveType(Message) (Components|GetOwner) "NewEnumerator2")
        (Components|Tick|SetComponentTickEnabled true)
        (return)
        (else
          (Utilities|PushFailInfo "Failed Attach Pushable Actor")
          (return))))
    (:else
      (return))))

(fn FindNearestAttachPointIndex
  (params (InPushableActor :type Actor%20Object%20Reference) (InPushAttachPoints :type Array%20of%20Transforms))
  (for (_array_element _array_index) InPushAttachPoints
    (LocalVariables|SetL_CurrentAttachPointIndex _array_index)
    (LocalVariables|SetL_CurrentAttachPointDistanceSq (Class|KismetMathLibrary|DistanceSquared2D (Math|Conversions|ToVector2D(Vector) (Math|Transform|TransformLocation (Transformation|GetActorTransform InPushableActor) (.location _array_element))) (Math|Conversions|ToVector2D(Vector) (Transformation|GetActorLocation (Components|GetOwner)))))
    (bind _interactraius (Class|BPICharacterState|GetCharacterInteractRadius(Message) (Components|GetOwner)))
    (if (> (Math|Float|Square _interactraius) (LocalVariables|GetL_CurrentAttachPointDistanceSq))
      (if (or (< (LocalVariables|GetL_CurrentAttachPointDistanceSq) (LocalVariables|GetL_NearestAttachPointDistanceSq)) (< (LocalVariables|GetL_NearestAttachPointIndex) 0))
        (LocalVariables|SetL_NearestAttachPointIndex (LocalVariables|GetL_CurrentAttachPointIndex))
        (LocalVariables|SetL_CurrentAttachPointDistanceSq (LocalVariables|GetL_NearestAttachPointDistanceSq)))))
  (return (LocalVariables|GetL_NearestAttachPointIndex)))

(fn CheckPushObstruction
  (bind _returnvalue (Components|GetOwner))
  (bind _returnvalue_2 (Components|GetOwner))
  (bind _array (Utilities|Array|MakeArray "ObjectTypeQuery1" "ObjectTypeQuery2"))
  (bind _currentactorpushing (Variables|Default|GetCurrentActorPushing))
  (bind _currentactorpushing_2 (Variables|Default|GetCurrentActorPushing))
  (bind _debug_status (Variables|Debug|GetDebug_Status))
  (bind _returnvalue_3 (Transformation|GetActorLocation _returnvalue_2))
  (bind _array_2 (Utilities|Array|MakeArray _currentactorpushing_2))
  (bind _returnvalue_4 (select _debug_status "ForOneFrame" "None"))
  (bind _pushablemesh (Variables|/Game/Blueprints/Environment/Carryable/BP_PushableBase.BP_PushableBase_C|GetPushableMesh _currentactorpushing))
  (bind _max (Components|StaticMesh|GetLocalBounds _pushablemesh))
  (bind _movedirection (Class|BPICharacterState|GetCharacterMoveDirection(Message) (Components|GetOwner)))
  (if (not (Utilities|Enum|Equal(Enum) (.StateMoveDirection (Utilities|Struct|BreakST_CharacterMoveDirection _movedirection)) "NewEnumerator8"))
    (bind _outhit (Class|KismetSystemLibrary|BoxTraceSingleforObjects (+ (Transformation|GetWorldLocation _pushablemesh) (* (+ (* (Transformation|GetActorForwardVector _returnvalue) (.Forward (Utilities|Struct|BreakST_CharacterMoveDirection _movedirection))) (* (Transformation|GetActorRightVector _returnvalue) (.Right (Utilities|Struct|BreakST_CharacterMoveDirection _movedirection)))) (.X (Math|Vector|BreakVector _max)))) (+ (Transformation|GetWorldLocation _pushablemesh) (* (+ (* (Transformation|GetActorForwardVector _returnvalue) (.Forward (Utilities|Struct|BreakST_CharacterMoveDirection _movedirection))) (* (Transformation|GetActorRightVector _returnvalue) (.Right (Utilities|Struct|BreakST_CharacterMoveDirection _movedirection)))) (.X (Math|Vector|BreakVector _max)))) (* _max (Transformation|GetWorldScale _pushablemesh)) (Transformation|GetWorldRotation _pushablemesh) _array false _array_2 _returnvalue_4 true "(R=0.173198,G=0.000000,B=1.000000,A=1.000000)" "(R=1.000000,G=0.012178,B=0.000000,A=1.000000)" 0.0))
    (if (or (.bBlockingHit (Collision|BreakHitResult _outhit)) (.bInitialOverlap (Collision|BreakHitResult _outhit)))
      (return "NewEnumerator1")
      (else
        (bind _outhit_2 (Collision|LineTraceForObjects (Math|Vector|MakeVector (.x _returnvalue_3) (.y _returnvalue_3) (.z _returnvalue_3)) (Transformation|GetWorldLocation (Variables|/Game/Blueprints/Environment/Carryable/BP_PushableBase.BP_PushableBase_C|GetPushableMesh (Variables|Default|GetCurrentActorPushing))) _array false _array_2 _returnvalue_4 true "(R=0.000000,G=0.051395,B=1.000000,A=1.000000)" "(R=1.000000,G=0.077227,B=0.000000,A=1.000000)" 0.0))
        (if (or (.bBlockingHit (Collision|BreakHitResult _outhit_2)) (.bInitialOverlap (Collision|BreakHitResult _outhit_2)))
          (return "NewEnumerator2")
          (else
            (return "NewEnumerator0")))))
    (else
      (return "NewEnumerator1"))))

(fn BeginInteractPush
  (params (InPushableActor :type BP%20Pushable%20Base%20Object%20Reference) (InPushAttachPoints :type Array%20of%20Transforms))
  (bind _nearestattachpointindex (Pushing|FindNearestAttachPointIndex InPushableActor InPushAttachPoints))
  (bind _returnvalue (Transformation|GetActorTransform InPushableActor))
  (bind _output (Utilities|Array|Get(acopy) InPushAttachPoints _nearestattachpointindex))
  (bind _returnvalue_2 (Math|Transform|ComposeTransforms _output _returnvalue))
  (LocalVariables|GetInPushableActor
    (:then
      (bind _success (Class|BPICharacterState|GetCharacterIsJumping(Message) (Components|GetOwner)))
      (if (not _success)
        (if (>= _nearestattachpointindex 0)
          (bind _halfheight (Class|BPICharacterState|GetCharacterHalfHeight(Message) (Components|GetOwner)))
          (bind _output_get (LocalVariables|SetL_CharacterHalfHeight _halfheight))
          (LocalVariables|SetL_TargetAttachPoint (Math|Transform|MakeTransform (+ (Math|Vector|MakeVector 0.0 0.0 _output_get) (.location _returnvalue_2)) (.rotation _returnvalue_2) (.scale _returnvalue_2)))
          (bind _characterradius (Class|BPICharacterState|GetCharacterRadius(Message) (Components|GetOwner)))
          (bind _outhit (Collision|CapsuleTraceByChannel (+ (.location (LocalVariables|GetL_TargetAttachPoint)) "0.000000,0.000000,70.000000") (+ (.location (LocalVariables|GetL_TargetAttachPoint)) "0.000000,0.000000,-100.000000") _characterradius (LocalVariables|GetL_CharacterHalfHeight) "TraceTypeQuery1" false (Utilities|Array|MakeArray InPushableActor) (select (Variables|Debug|GetDebug_Status) "ForDuration" "None") true "(R=0.164130,G=0.000000,B=1.000000,A=1.000000)" "(R=1.000000,G=0.103472,B=0.000383,A=1.000000)" 2.0))
          (if (not (.bInitialOverlap (Collision|BreakHitResult _outhit)))
            (bind _walkablefloorz (Class|BPICharacterState|GetCharacterWalkableFloorZ(Message) (Components|GetOwner)))
            (if (< _walkablefloorz (.Z (Math|Vector|BreakVector (.ImpactNormal (Collision|BreakHitResult _outhit)))))
              (bind _returnvalue_3 (Collision|LineTraceByChannel (Transformation|GetActorLocation InPushableActor) (.location (LocalVariables|GetL_TargetAttachPoint)) "TraceTypeQuery1" false (Utilities|Array|MakeArray InPushableActor) (select (Variables|Debug|GetDebug_Status) "ForDuration" "None") true "(R=0.084027,G=0.000000,B=1.000000,A=1.000000)" "(R=1.000000,G=0.061766,B=0.000000,A=1.000000)" 2.0))
              (if (not _returnvalue_3)
                (Class|BPICharacterState|ResetSpeedandJump(Message) (Components|GetOwner) false)
                (bind _success_2 (Class|BPICharacterState|SetCharacterTransform(Message) (Components|GetOwner) (LocalVariables|GetL_TargetAttachPoint)))
                (if _success_2
                  (Variables|Default|SetCurrentActorPushing InPushableActor)
                  (Pushing|StartPushing)
                  (return true)
                  (else
                    (Utilities|PushFailInfo "Не смогли переместить персонажа")
                    (return false)))
                (else
                  (Utilities|PushFailInfo "Между персонажем и объектом стена")
                  (return false)))
              (else
                (Utilities|PushFailInfo "Некуда расположить персонажа")
                (return false)))
            (else
              (Utilities|PushFailInfo "Нет места для персонажа")
              (return false)))
          (else
            (Utilities|PushFailInfo "Не найдено точек крепления")
            (return false)))
        (else
          (Utilities|PushFailInfo "Персонаж в прыжке")
          (return false))))
    (:else
      (return false))))

(fn DebugCheckIsItem
  (return false))

(fn DebugGetItemDetails
  (return ""))

(fn DebugGetOverlappedActors
  (return 0))

(fn DebugGetStatus
  (return (Variables|Debug|GetDebug_Status)))

(fn DebugSetStatus
  (params (DebugStatus :type Boolean))
  (bind _output_get (Variables|Debug|SetDebug_Status DebugStatus))
  (return _output_get))

(fn DebugSetVisibilityInteractCollision
  (params (SetVisibility :type Boolean))
  (return false))

(fn EndInteractPush
  (params (InCurrentPushableActor :type Actor%20Object%20Reference))
  (if (and (== InCurrentPushableActor (Variables|Default|GetCurrentActorPushing)) (Utilities|IsValid (Variables|Default|GetCurrentActorPushing)))
    (Class|BPICharacterState|ResetSpeedandJump(Message) (Components|GetOwner) false)
    (Transformation|DetachFromActor (Variables|Default|GetCurrentActorPushing) "KeepWorld" "KeepWorld" "KeepWorld")
    (Components|Tick|SetComponentTickEnabled false)
    (Class|BPICharacterState|SwitchCharacterMoveType(Message) (Components|GetOwner) "NewEnumerator0")
    (Variables|Default|SetCurrentActorPushing 0)
    (return false)
    (else
      (return false))))

(fn GetCharacterIsPush
  (Variables|Default|GetCurrentActorPushing
    (:then
      (return true))
    (:else
      (return false))))