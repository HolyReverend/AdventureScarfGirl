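; Lock component that gates an interactable, such as a door, behind key items held by the player.
; CheckKeys matches player item names against KeyNeeds, removes the keys when all are found and changes LockedType, calling DoorLockStatus for empty inventory, missing keys or success.
; GetLockedCondition runs that check and returns true only if it succeeds and IsImmediatelyOpen also passes.
; The remaining interaction functions are stubs returning fixed or empty values.
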(fn CheckKeys
  (bind _items (Class|BPIBackpack|GetItemsfromCharacter(Message) (CallFunction|GetActualPlayer)))
  (if (Utilities|Array|IsNotEmpty _items)
    (LocalVariables|SetL_NumberNeedKeys (Utilities|Array|Length (Variables|Default|GetKeyNeeds)))
    (bind _array_element (Utilities|Array|ForEachLoopwithBreak _items :!label _label)
      (:LoopBody
        (bind _output_get (LocalVariables|SetL_FindItem _array_element))
        (if (Utilities|Array|ContainsItem (Variables|Default|GetKeyNeeds) (Utilities|Struct|BreakST_ItemDetails _output_get))
          (Utilities|Array|AddUnique (LocalVariables|GetL_FindNeedItems) (LocalVariables|GetL_FindItem))
          (bind _result (Math|Integer|DecrementInt (LocalVariables|GetL_NumberNeedKeys))
            (:%20%20
              (if (== _result 0)
                (goto _label Break))))))
      (:Completed
        (if (== (LocalVariables|GetL_NumberNeedKeys) 0)
          (bind _success (Class|BPIBackpack|RemoveItemfromCharacter(Message) (CallFunction|GetActualPlayer) (LocalVariables|GetL_FindNeedItems)))
          (if _success
            (Default|CallDoorLockStatus "NewEnumerator2")
            (bind _succes (CallFunction|SetLockedType "NewEnumerator0"))
            (if _succes
              (return true)
              (else
                (return false)))
            (else
              _))
          (else
            (Default|CallDoorLockStatus "NewEnumerator1")))
        (return false)))
    (else
      (Default|CallDoorLockStatus "NewEnumerator0")
      (return false))))

(fn GetDelayInteractHandlerValidate
  (return false))

(fn GetInteractStatus
  (return "NewEnumerator2"))

(fn GetIsTriggerActor
  (return false))

(fn GetLockedCondition
  (bind _succes (CallFunction|CheckKeys))
  (if _succes
    (Variables|Default|GetIsImmediatelyOpen
      (:then
        (return true))
      (:else
        (return false)))
    (else
      (return false))))

(fn GetLockedType
  (return (Variables|Default|GetLockedType)))

(fn GetReturnInteractHandlerValidate
  (return false))

(fn GetReturnTimeValid
  (return false))

(fn GetReturnTotalDelayTime
  (return 0.0))

(fn GetTriggeredActors
  (return 0))

(fn SetInteractableState
  (params (State :type E_InteractableState%20Enum :default "NewEnumerator0"))
  (return false))

(fn SetLockedType
  (params (InLockedType :type E_InteractLockedType%20Enum :default "NewEnumerator0"))
  (Variables|Default|SetLockedType InLockedType)
  (return true))

(fn StartInteract
  (params (InActor :type Actor%20Object%20Reference))
  (return false))