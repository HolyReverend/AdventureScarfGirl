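; BPC_PlayerDebuger is a debug component for the player character, driven by numpad hotkeys.
; BeginPlay enables input through the first player controller, and Tick prints an on-screen Russian hint about enabling debug while DebugEnable is unset.
; Num 0 flips DebugEnable through a FlipFlop with empty branches.
; Num 1 calls StartInteractMessage on the BP_DoorBase returned by GetActorOfClass, regardless of the debug toggle.
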(event EventBeginPlay
  (bind _returnvalue (Game|GetPlayerController 0))
  (|CallParentFunction)
  (Input|EnableInput _returnvalue _returnvalue))

(event EventTick
  (params (DeltaSeconds :type Float%20%28single-precision%29))
  (|CallParentFunction DeltaSeconds)
  (Variables|Default|GetDebugEnable
    (:then)
    (:else
      (Development|PrintString (Utilities|String|Append "Включить дебаг персонажа: " "Num 0") true false "(R=1.000000,G=0.083948,B=0.000000,A=1.000000)" 0.0))))

(event Input|KeyboardEvents|DebugKeyNumPadZero
  (params (Key :type Key%20Structure :default "None") (ActionValue :type Input%20Action%20Value%20Structure))
  (:Pressed
    (bind _isa (Utilities|FlowControl|FlipFlop)
      (:A
        _)
      (:B
        _))
    (Variables|Default|SetDebugEnable _isa)))

(event Input|KeyboardEvents|DebugKeyNumPadOne
  (params (Key :type Key%20Structure :default "None") (ActionValue :type Input%20Action%20Value%20Structure))
  (:Pressed
    (bind _returnvalue (Actor|GetActorOfClass "/Game/Blueprints/Environment/Doors/BP_DoorBase.BP_DoorBase_C"))
    (Class|BPIInteracable|StartInteract(Message) _returnvalue)))