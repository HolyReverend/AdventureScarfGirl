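; Debug component for interactable actors that prints their state on screen, with Russian text.
; BeginPlay uses the enable flag to set tick, notify the owner and apply collision visibility, and binds to BP_DoorLock status events for item-requirement results.
; Tick prints the owner's item details or interact status, plus overlapping actors, naming only BPI_SaveLoadData implementers.
; Owner data comes through message calls, with separate flags gating each printout.
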(event EventBeginPlay
  (bind _debugenablecomponent (Variables|Default|GetDebugEnableComponent))
  (|CallParentFunction)
  (Components|Tick|SetComponentTickEnabled (Variables|Default|GetDebugEnableComponent))
  (Class|BPIDebuger|DebugSetStatus(Message) (Components|GetOwner) _debugenablecomponent)
  (if _debugenablecomponent
    (Utilities|FlowControl|Sequence
      (:then_0
        (Class|BPIDebuger|DebugSetVisibilityInteractCollision(Message) (Components|GetOwner) (Variables|Settings|General|GetSetVisibilityInteractCollision)))
      (:then_1
        (if (Variables|Settings|Status|GetDebugInteractStatus)
          (bind _asbp_door_lock (Utilities|Casting|CastToBP_DoorLock (Components|GetOwner)))
          (EventDispatchers|BindEventtoDoorLockStatus _asbp_door_lock (EventDispatchers|CreateEvent :!event PrintDoorLockStatus)))))))

(event EventTick
  (params (DeltaSeconds :type Float%20%28single-precision%29))
  (|CallParentFunction DeltaSeconds)
  (if (Variables|Default|GetDebugEnableComponent)
    (Utilities|FlowControl|Sequence
      (:then_0
        (CallFunction|PrintInteractStatus))
      (:then_1
        (CallFunction|PrintActorInsideCollision)))))

(fn PrintInteractStatus
  (if (Variables|Settings|Status|GetDebugInteractStatus)
    (bind _succes (Class|BPIDebuger|DebugCheckIsItem(Message) (Components|GetOwner)))
    (if _succes
      (bind _itemdetalis (Class|BPIDebuger|DebugGetItemDetails(Message) (Components|GetOwner)))
      (Development|PrintText (Utilities|Text|FormatText "Тип: {type}; Название: {name}; Описание: {description}" (|GenerictoText (.ItemType (Utilities|Struct|BreakST_ItemDetails _itemdetalis))) (|GenerictoText (.ItemName (Utilities|Struct|BreakST_ItemDetails _itemdetalis))) (.ItemDescription (Utilities|Struct|BreakST_ItemDetails _itemdetalis))) true false "(R=0.000000,G=0.155926,B=0.127438,A=1.000000)" 0.0)
      (return)
      (else
        (bind _interactablestatus (Class|BPIInteractable|GetInteractStatus(Message) (Components|GetOwner)))
        (Development|PrintText (Utilities|Text|FormatText "Состояние {interactObject}: {Status}" (Components|GetOwner) (Utilities|String|EnumtoString _interactablestatus)) true false "(R=0.000000,G=0.155926,B=0.127438,A=1.000000)" 0.0)
        (return)))
    (else
      (return))))

(fn PrintActorInsideCollision
  (if (Variables|Settings|Status|GetDebugActorInsideCollision)
    (bind _actor (Class|BPIDebuger|DebugGetOverlappedActors(Message) (Components|GetOwner)))
    (if (Utilities|Array|IsNotEmpty _actor)
      (for _array_element _actor
        (Development|PrintText (Utilities|Text|FormatText "В зоне {interactableObject} находится: {actor}" (Components|GetOwner) (Utilities|String|SelectText (Utilities|Text|ToText(Object) _array_element) "Никого" (Utilities|DoesObjectImplementInterface _array_element "/Game/Blueprints/Interfaces/System/BPI_SaveLoadData.BPI_SaveLoadData_C"))) true false "(R=0.000000,G=0.660000,B=1.000000,A=1.000000)" 0.0))
      (else
        (Development|PrintText (Utilities|Text|FormatText "В зоне {interactableObject} никого нет" (Components|GetOwner)) true false "(R=0.000000,G=0.660000,B=1.000000,A=1.000000)" 0.0)))
    (return)
    (else
      (return))))

(fn PrintDoorLockStatus
  (params (NewParam :type E_InteractLockedStatus%20Enum :default "NewEnumerator0"))
  (CallFunction|PrintSeparator 5.0)
  (switch Utilities|FlowControl|Switch|SwitchonE_InteractLockedStatus NewParam
    (:NewEnumerator0
      (Development|PrintText (Utilities|Text|FormatText "Для объекта {actor} нет необходимых предметов" (Components|GetOwner)) true true "(R=0.040625,G=0.040625,B=0.040625,A=1.000000)" 5.0))
    (:NewEnumerator1
      (Development|PrintText (Utilities|Text|FormatText "Для объекта {actor} недостаточно предметов" (Components|GetOwner)) true true "(R=0.040625,G=0.040625,B=0.040625,A=1.000000)" 5.0))
    (:NewEnumerator2
      (Development|PrintText (Utilities|Text|FormatText "Для объекта {actor} все предметы переданы!" (Components|GetOwner)) true true "(R=0.040625,G=0.040625,B=0.040625,A=1.000000)" 5.0))))