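; Text render component that shows a "Press {button}" world hint for an interactable owner, using the key mapped to its input action.
; It starts hidden and binds to the owner's interaction component through interface messages, toggling visibility by whether the player is inside its collision.
; Each tick it can rotate toward that player's camera.
; A use flash steps back along a color curve on a looping timer.
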(event EventBeginPlay
  (Rendering|SetVisibility false true)
  (ColorFlashing|BindHintUse)
  (Utilities|FlowControl|Delay 1.0)
  (CallFunction|ConfigureKeyDisplay))

(event EventTick
  (params (DeltaSeconds :type Float%20%28single-precision%29))
  (RotateHint|LookingatPlayerCamera))

(fn ConfigureKeyDisplay
  (bind _playercontrollkeys (Class|BPIPlayerControllerState|GetPlayerControllKeys(Message) (Game|GetPlayerController 0)))
  (bind _array_element (Utilities|Array|ForEachLoopwithBreak _playercontrollkeys :!label _label)
    (:LoopBody
      (if (== (.InputAction (Utilities|Struct|BreakST_PlayerControlKeys _array_element)) (Variables|KeyMapped|GetIA_Action))
        (goto _label Break)))
    (:Completed
      (Rendering|Components|TextRender|SetText (Utilities|Text|FormatText "Press {button}" (Class|KismetInputLibrary|KeyGetDisplayName (.Key (Utilities|Struct|BreakST_PlayerControlKeys _array_element)) true)))
      (Default|CallKeyTextObtained))))

(fn BindHintUse
  (bind _owner (Class|BPIInteractable|GetOwnerBPC(Message) (Components|GetOwner)))
  (EventDispatchers|BindEventtoBeginUse _owner (EventDispatchers|CreateEvent :!event StartingUse))
  (EventDispatchers|BindEventtoOnInteractionUseReady _owner (EventDispatchers|CreateEvent :!event InteractionUseReady)))

(fn StartingUse
  (bind _output_get (Variables|ColorFlashing|SetHintColorTIme 1.0))
  (Rendering|Components|TextRender|SetTextRenderColor self (Math|Conversions|ToColor(LinearColor) (Math|Curves|GetLinearColorValue (Variables|ColorFlashing|GetHintCurveColor) _output_get)))
  (bind _returnvalue (Utilities|Time|SetTimerbyEvent (EventDispatchers|CreateEvent :!event HintColorChangeRevert) 0.1 true))
  (Variables|ColorFlashing|SetHintColorTimeHandler _returnvalue))

(fn HintColorChangeRevert
  (if (>= (Variables|ColorFlashing|GetHintColorTIme) 0.0)
    (Rendering|Components|TextRender|SetTextRenderColor self (Math|Conversions|ToColor(LinearColor) (Math|Curves|GetLinearColorValue (Variables|ColorFlashing|GetHintCurveColor) (Variables|ColorFlashing|GetHintColorTIme))))
    (Variables|ColorFlashing|SetHintColorTIme (- (Variables|ColorFlashing|GetHintColorTIme) 0.1))
    (else
      (Utilities|Time|ClearandInvalidateTimerbyHandle (Variables|ColorFlashing|GetHintColorTimeHandler))
      (Variables|ColorFlashing|SetHintColorTIme 0.0))))

(fn LookingatPlayerCamera
  (Variables|General|GetisHintTextEnable
    (:then
      (Variables|GetbVisible
        (:then
          (Variables|General|GetIsHintTextRotate
            (:then
              (bind _owner (Class|BPIInteractable|GetOwnerBPC(Message) (Components|GetOwner)))
              (if (.Success (Default|CheckPlayerInsideCollision _owner))
                (bind _playercamera (Class|BPICharacterState|GetPlayerCameraTransform(Message) (.PlayerCharacter (Default|CheckPlayerInsideCollision _owner))))
                (LocalVariables|SetL_CameraLocation (.Location (Math|Transform|BreakTransform _playercamera)))
                (Transformation|SetWorldRotation (Math|Rotator|FindLookatRotation (Transformation|GetWorldLocation) (LocalVariables|GetL_CameraLocation)) false false)
                (return)
                (else
                  (return))))
            (:else
              (return))))
        (:else
          (return))))
    (:else
      (return))))

(fn InteractionUseReady
  (Variables|General|GetisHintTextEnable
    (:then
      (bind _owner (Class|BPIInteractable|GetOwnerBPC(Message) (Components|GetOwner)))
      (Rendering|SetVisibility (.Success (Default|CheckPlayerInsideCollision _owner)) true)
      (return))
    (:else
      (return))))