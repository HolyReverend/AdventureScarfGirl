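; BPC_DebugerBase is a debug component that prints on-screen diagnostics about its owning actor.
; While enabled, each Tick it prints a separator and an owner "debug enabled" line, then an optional velocity line in a configurable color.
; The velocity text comes from the owner's DebugGetVelocityMessage.
; Messages are in Russian, with zero duration to refresh every frame, and the text lines skip the log.
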(event EventBeginPlay)

(event EventTick
  (params (DeltaSeconds :type Float%20%28single-precision%29))
  (if (Variables|Settings|General|GetDebugEnableComponent)
    (CallFunction|PrintOwnerDebugEnabled)
    (CallFunction|PrintVelocity)))

(fn PrintVelocity
  (bind _returnvalue (Components|GetOwner))
  (if (Variables|Settings|Velocity|GetDebugVelocityEnable)
    (bind _velocity (Class|BPIDebuger|DebugGetVelocity(Message) _returnvalue))
    (Development|PrintText (Utilities|Text|FormatText "Скорость \"{owner}\": {velocity}" _returnvalue _velocity) true false (Variables|Settings|Velocity|GetDebugVelocityColor) 0.0)
    (return)
    (else
      (return))))

(fn PrintOwnerDebugEnabled
  (CallFunction|PrintSeparator 0.0)
  (Development|PrintText (Utilities|Text|FormatText "Debug включён для: {owner}" (Components|GetOwner)) true false "(R=0.000000,G=0.396755,B=0.896269,A=1.000000)" 0.0)
  (return))