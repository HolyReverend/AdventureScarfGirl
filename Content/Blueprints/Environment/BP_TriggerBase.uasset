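; Base trigger interactable that relays interaction to the actors in its TriggeredActors list, removing itself from that list on BeginPlay.
; It extends the parent's interact logic, gating it on overlap checks and the targets' interact status.
; StartInteract and Overlap-type interactions either fire the targets at once or bind to an end-move event to fire them later, depending on StartImmediately.
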(event Custom|StartDefferedInteract
  (Interaction|StartInteractwithActor))

(event EventTick
  (params (DeltaSeconds :type Float%20%28single-precision%29))
  (|CallParentFunction DeltaSeconds))

(event EventInteracttoObject
  (Variables|Settings|GetCheckAvailableInteractActor
    (:then
      (if (CallFunction|CheckCanIsInteract (CallFunction|GetOverlappedActor) false)
        (bind _succes (Interaction|GetAvailableInteractActor))
        (if _succes
          (|CallParentFunction :!label _label)
          (switch Utilities|FlowControl|Switch|SwitchonE_InteractType (Variables|Default|GetInteractType)
            (:NewEnumerator0
              (Variables|Settings|GetStartImmediately
                (:then
                  (Interaction|StartInteractwithActor))
                (:else
                  (EventDispatchers|AssignEndMoveInteract (delegate Custom|StartDefferedInteract)))))))
        (else
          (goto _label))))
    (:else
      (goto _label))))

(event EventBeginPlay
  (|CallParentFunction)
  (CallFunction|RemoveSelffromTriggeredArray))

(fn ConstructionScript
  (|CallParentFunction))

(fn StartInteract
  (params (InActor :type Actor%20Object%20Reference))
  (bind _succes (|CallParentFunction InActor))
  (if _succes
    (Variables|Settings|GetStartImmediately
      (:then
        (Interaction|StartInteractwithActor)
        (return true))
      (:else
        (EventDispatchers|BindEventtoEndMoveInteract (EventDispatchers|CreateEvent :!event Custom|StartDefferedInteract))))
    (else
      (return false))))

(fn StartInteractwithActor
  (for _array_element (Variables|Settings|GetTriggeredActors)
    (CallFunction|StartInteract _array_element self))
  (return))

(fn GetAvailableInteractActor
  (if (Utilities|Array|IsNotEmpty (Variables|Settings|GetTriggeredActors))
    (bind _array_element (Utilities|Array|ForEachLoopwithBreak (Variables|Settings|GetTriggeredActors) :!label _label)
      (:LoopBody
        (Utilities|IsValid _array_element
          (:Is%20Valid
            (bind _interactablestatus (Default|GetInteractStatus _array_element))
            (if (Utilities|Enum|Equal(Enum) _interactablestatus "NewEnumerator0")
              (goto _label Break)))))
      (:Completed
        (bind _interactablestatus_2 (Default|GetInteractStatus _array_element))
        (if (not (Utilities|Enum|Equal(Enum) _interactablestatus_2 "NewEnumerator0"))
          (return true)
          (else
            (return false)))))
    (else
      (return false))))

(fn GetIsTriggerActor
  (return true))

(fn RemoveSelffromTriggeredArray
  (bind _array_element (Utilities|Array|ForEachLoopwithBreak (Variables|Settings|GetTriggeredActors) :!label _label)
    (:LoopBody
      (if (== _array_element self)
        (goto _label Break)))
    (:Completed
      (Utilities|Array|RemoveItem (Variables|Settings|GetTriggeredActors) self)
      (return))))

(fn GetTriggeredActors
  (return (Variables|Settings|GetTriggeredActors)))