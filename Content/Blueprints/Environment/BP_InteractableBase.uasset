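; Base Blueprint for interactable world objects, with an empty InteractToObject event and stub getters for children to override.
; InteractCollision tracks filtered overlapping actors; enabled Overlap types fire InteractToObject on first entry and last exit.
; Use types instead toggle HintScene, rotated toward the player camera on Tick, and fire through StartInteract.
; InteractableState (Enable, Trigger, Disable) gates interaction and which actor type StartInteract accepts.
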(event OnComponentBeginOverlap(InteractCollision)
  (params (OverlappedComponent :type Primitive%20Component%20Object%20Reference) (OtherActor :type Actor%20Object%20Reference) (OtherComp :type Primitive%20Component%20Object%20Reference) (OtherBodyIndex :type Integer) (bFromSweep :type Boolean) (SweepResult :type Hit%20Result%20Structure%20%28by%20ref%29))
  (bind _succes (CallFunction|ActorEnter OtherActor true))
  (if _succes
    (CallFunction|InteracttoObject)))

(event OnComponentEndOverlap(InteractCollision)
  (params (OverlappedComponent :type Primitive%20Component%20Object%20Reference) (OtherActor :type Actor%20Object%20Reference) (OtherComp :type Primitive%20Component%20Object%20Reference) (OtherBodyIndex :type Integer))
  (bind _succes (CallFunction|ActorEnter OtherActor false))
  (if _succes
    (CallFunction|InteracttoObject)))

(event Custom|InteractToObject)

(event EventBeginPlay
  (Rendering|SetVisibility (Variables|Default|GetHintScene) false true))

(event EventTick
  (params (DeltaSeconds :type Float%20%28single-precision%29))
  (HintKey|LookingatPlayerCamera))

(fn ConstructionScript
  (Components|Box|SetBoxExtent (Variables|Default|GetInteractCollision) (Variables|Settings|General|GetInteractCollisionBox) true)
  (Rendering|SetVisibility (Variables|Default|GetHintScene) (Utilities|Select :Index (Variables|Settings|Type|GetInteractType) :NewEnumerator0 false :NewEnumerator1 true) true))

(fn ActorEnter
  (params (InOverlapperActor :type Actor%20Object%20Reference) (IsActorEnter :type Boolean))
  (if (CallFunction|CheckCanIsInteract InOverlapperActor (Variables|Settings|General|GetTargetActorType))
    (Utilities|Array|AddUnique (Variables|Default|GetOverlapActors) InOverlapperActor)
    (bind _succes (CallFunction|GetIsTriggerActor))
    (if _succes
      (bind _triggeredactors (CallFunction|GetTriggeredActors))
      (if (Utilities|Array|IsNotEmpty _triggeredactors)
        _
        (else
          (return false))))
    (if IsActorEnter
      (Variables|Default|GetIsActorInsideCollision
        (:then
          (return false))
        (:else
          (Default|CallBeginFirstOverlap)))
      (else
        (Utilities|Array|RemoveItem (Variables|Default|GetOverlapActors) InOverlapperActor)
        (if (Utilities|Array|IsEmpty (Variables|Default|GetOverlapActors))
          (Variables|Default|GetIsActorInsideCollision
            (:then
              (Default|CallEndLastOverlap))
            (:else
              (return false)))
          (else
            (return false)))))
    (Variables|Default|SetIsActorInsideCollision IsActorEnter)
    (switch Utilities|FlowControl|Switch|SwitchonE_InteractableState (Variables|Settings|General|GetInteractableState)
      (:NewEnumerator0
        (switch Utilities|FlowControl|Switch|SwitchonE_InteractType (Variables|Settings|Type|GetInteractType)
          (:NewEnumerator0
            (return true))
          (:NewEnumerator1
            (HintKey|InteractionHint)
            (return false))))
      (:NewEnumerator3
        _)
      (:NewEnumerator1
        _))
    (return false)
    (else
      (return false))))

(fn GetOverlappedActor
  (if (Utilities|Array|IsNotEmpty (Variables|Default|GetOverlapActors))
    (return (Utilities|Array|Get(acopy) (Variables|Default|GetOverlapActors)))
    (else
      (return 0))))

(fn GetIsActorInsideCollision
  (return (Variables|Default|GetIsActorInsideCollision)))

(fn GetInteractInstigator
  (return (Variables|Default|GetInteractInstigator)))

(fn InteractionHint
  (Rendering|SetVisibility (Variables|Default|GetHintScene) (.Success (CallFunction|CheckPlayerInsideCollision)) true))

(fn CheckPlayerInsideCollision
  (bind _array_element (Utilities|Array|ForEachLoopwithBreak (Variables|Default|GetOverlapActors) :!label _label)
    (:LoopBody
      (if (== _array_element (CallFunction|GetActualPlayer))
        (LocalVariables|SetL_PlayerFound true)
        (goto _label Break)))
    (:Completed
      (return (LocalVariables|GetL_PlayerFound) _array_element))))

(fn LookingatPlayerCamera
  (bind (_success _playercharacter) (CallFunction|CheckPlayerInsideCollision))
  (Variables|/Script/Engine.SceneComponent|GetbVisible (Variables|Default|GetHintScene)
    (:then
      (if _success
        (bind _playercamera (Class|BPICharacterState|GetPlayerCameraTransform(Message) _playercharacter))
        (LocalVariables|SetL_CameraLocation (.Location (Math|Transform|BreakTransform _playercamera)))
        (Transformation|SetWorldRotation (Variables|Default|GetHintScene) (Math|Rotator|FindLookatRotation (Transformation|GetWorldLocation (Variables|Default|GetHintScene)) (LocalVariables|GetL_CameraLocation)) false false)
        (return)))
    (:else
      (return))))

(fn DebugCheckIsItem
  (return false))

(fn DebugGetItemDetails
  (return ""))

(fn DebugGetOverlappedActors
  (return (Variables|Default|GetOverlapActors)))

(fn DebugSetVisibilityInteractCollision
  (params (SetVisibility :type Boolean))
  (Development|SetHiddeninGame (Variables|Default|GetInteractCollision) (not SetVisibility) false)
  (return true))

(fn GetDelayInteractHandlerValidate
  (return false))

(fn GetInteractStatus
  (return (Variables|Settings|General|GetInteractStatus)))

(fn GetIsTriggerActor
  (return false))

(fn GetLockedType
  (return "NewEnumerator0"))

(fn GetReturnInteractHandlerValidate
  (return false))

(fn GetReturnTimeValid
  (return false))

(fn GetReturnTotalDelayTime
  (return 0.0))

(fn GetTriggeredActors
  (return 0))

(fn SetInteractableState
  (params (State :type E_InteractableState%20Enum :default "NewEnumerator0"))
  (Variables|Settings|General|SetInteractableState State)
  (return true))

(fn SetLockedType
  (params (InLockedType :type E_InteractLockedType%20Enum :default "NewEnumerator0"))
  (return false))

(fn StartInteract
  (params (InActor :type Actor%20Object%20Reference))
  (switch Utilities|FlowControl|Switch|SwitchonE_InteractableState (Variables|Settings|General|GetInteractableState)
    (:NewEnumerator0
      (if (CallFunction|CheckCanIsInteract InActor "NewEnumerator0")
        _
        (else
          (return false))))
    (:NewEnumerator3
      (if (CallFunction|CheckCanIsInteract InActor "NewEnumerator2")
        _
        (else
          (return false))))
    (:NewEnumerator1
      (return false)))
  (CallFunction|InteracttoObject)
  (switch Utilities|FlowControl|Switch|SwitchonE_InteractType (Variables|Settings|Type|GetInteractType)
    (:NewEnumerator0
      _)
    (:NewEnumerator1
      (Variables|Default|SetInteractInstigator InActor)))
  (return true))