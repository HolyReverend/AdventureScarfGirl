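; Base Blueprint for interactable mechanism beam objects in the environment, providing shared ray data and hooks.
; The construction script caches a beam ray struct from the arrow's location and forward vector, max distance, and the movable mesh's scaled bounds and rotation.
; Interaction calls the parent, then an empty TryInteractMechBeam event.
; Receiver check, activation getter and setter are stubs returning false, while GetMechBeamRay exposes the cached ray.
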(event Custom|TryInteractMechBeam)

(event EventInteracttoObject
  (|CallParentFunction)
  (CallFunction|TryInteractMechBeam))

(fn ConstructionScript
  (|CallParentFunction)
  (Beam|Construct|ConstructBeamData))

(fn ConstructBeamData
  (CallFunction|SetActualMechBeamRay)
  (return))

(fn SetActualMechBeamRay
  (bind _mavablemesh (Variables|Default|GetMavableMesh))
  (bind _arrow (Variables|Default|GetArrow))
  (Variables|Default|SetMechBeamRay (Utilities|Struct|MakeST_MechanismBeamRay (Transformation|GetWorldLocation _arrow) (Math|Vector|GetForwardVector _arrow) (Variables|Beam|GetBeamMaxDistance) (* (.Max (Components|StaticMesh|GetLocalBounds _mavablemesh)) (Variables|Beam|GetWidthSizeMod)) (Transformation|GetWorldRotation _mavablemesh)))
  (return))

(fn CheckIsMechBeamReceiver
  (params (inActor :type Actor%20Object%20Reference))
  (return false))

(fn GetMechBeamActivated
  (return false))

(fn GetMechBeamRay
  (return (Variables|Default|GetMechBeamRay)))

(fn SetMechBeamActivate
  (params (OnActivate :type Boolean))
  (return false))