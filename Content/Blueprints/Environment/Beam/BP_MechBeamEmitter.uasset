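; Puzzle beam emitter that, when the player interacts, tries to chain a beam through its assigned mirror network to a receiver.
; Box traces hop between unvisited network mirrors, with timers delaying each hop by distance over beam speed.
; Reaching a receiver changes the emitter's and network's interactable state; any invalid hit resets the attempt.
; An optional construction-script preview draws the traces as debug boxes.
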(event Custom|StartBuildNetworkBeam
  (CallFunction|RebuildBeam self))

(event EventTryInteractBeamEmitter
  (|CallParentFunction)
  (if (== (CallFunction|GetInteractInstigator) (CallFunction|GetActualPlayer))
    (Variables|Default|GetIsBusy
      (:then
        (if (CallFunction|GetDebugStatus)
          (Development|PrintString "Эмиттор занят!" true false "(R=0.258183,G=0.000911,B=0.000911,A=1.000000)" 5.0)))
      (:else
        (Default|CallMechBeamNetworkChange)
        (Variables|Default|SetIsBusy true)))))

(event EventBeginPlay
  (|CallParentFunction)
  (if (Utilities|Array|IsNotEmpty (Variables|Beam|GetMechBeamMirrorNetwork))
    (EventDispatchers|BindEventtoMechBeamNetworkChange (delegate Custom|StartBuildNetworkBeam))))

(fn ConstructionScript
  (|CallParentFunction)
  (Construct|BuildMirrorNetworkPreview))

(fn RebuildBeam
  (params (InActor :type Actor%20Object%20Reference))
  (bind _beamray (Class|BPIMechanismBeam|GetMechBeamRay(Message) InActor))
  (bind _outhit (Collision|BoxTraceByChannel (.Start (Utilities|Struct|BreakST_MechanismBeamRay _beamray)) (+ (.Start (Utilities|Struct|BreakST_MechanismBeamRay _beamray)) (* (.Direction (Utilities|Struct|BreakST_MechanismBeamRay _beamray)) (.BeamMaxDistance (Utilities|Struct|BreakST_MechanismBeamRay _beamray)))) (.BeamSize (Utilities|Struct|BreakST_MechanismBeamRay _beamray)) (.BeamRotation (Utilities|Struct|BreakST_MechanismBeamRay _beamray)) "TraceTypeQuery3" false (Utilities|Array|MakeArray InActor) (select (CallFunction|GetDebugStatus) "ForDuration" "None") true "(R=0.095695,G=0.000000,B=1.000000,A=1.000000)" "(R=1.000000,G=0.103386,B=0.000000,A=1.000000)"))
  (bind _output_get (LocalVariables|SetL_FindedMechBeamMirror (.HitActor (Collision|BreakHitResult _outhit))))
  (if (not (Utilities|Array|ContainsItem (Variables|Default|GetUsedMechBeamMirrors) _output_get))
    (LocalVariables|SetL_FindedMechBeamMirrorDistance (.Distance (Collision|BreakHitResult _outhit)))
    (if (Utilities|DoesObjectImplementInterface (LocalVariables|GetL_FindedMechBeamMirror) "/Game/Blueprints/Interfaces/Interactable/BPI_MechanismBeam.BPI_MechanismBeam_C")
      (bind _success (Class|BPIMechanismBeam|CheckIsMechBeamReceiver(Message) (LocalVariables|GetL_FindedMechBeamMirror) (LocalVariables|GetL_FindedMechBeamMirror)))
      (if _success
        (CallFunction|SuccesCreateMirrorNetwork)
        (return)
        (else
          (bind _array_element (Utilities|Array|ForEachLoopwithBreak (Variables|Beam|GetMechBeamMirrorNetwork) :!label _label)
            (:LoopBody
              (if (== _array_element (LocalVariables|GetL_FindedMechBeamMirror))
                (Utilities|Array|AddUnique (Variables|Default|GetUsedMechBeamMirrors) (LocalVariables|GetL_FindedMechBeamMirror))
                (LocalVariables|SetL_MechBeamRecieverFound true)
                (goto _label Break)))
            (:Completed
              (LocalVariables|GetL_MechBeamRecieverFound
                (:then
                  (Variables|Default|SetNextMechBeamMirror (LocalVariables|GetL_FindedMechBeamMirror))
                  (Utilities|Time|SetTimerbyEvent (EventDispatchers|CreateEvent :!event NextMirrorFounded) (/ (LocalVariables|GetL_FindedMechBeamMirrorDistance) (Variables|Beam|GetBeamSpeed)))
                  (return))
                (:else
                  (CallFunction|ClearMirrorNetwork)
                  (return)))))))
      (else
        (CallFunction|ClearMirrorNetwork)
        (return)))
    (else
      (CallFunction|ClearMirrorNetwork)
      (return))))

(fn NextMirrorFounded
  (CallFunction|RebuildBeam (Variables|Default|GetNextMechBeamMirror))
  (return))

(fn ClearMirrorNetwork
  (Utilities|Array|Clear (Variables|Default|GetUsedMechBeamMirrors))
  (Variables|Default|SetNextMechBeamMirror 0)
  (Variables|Default|SetIsBusy false)
  (return))

(fn SuccesCreateMirrorNetwork
  (for _array_element (Variables|Beam|GetMechBeamMirrorNetwork)
    (Default|SetInteractableState _array_element "NewEnumerator1"))
  (Default|SetInteractableState self "NewEnumerator1")
  (CallFunction|ClearMirrorNetwork)
  (return))

(fn BuildMirrorNetworkPreview
  (Variables|Beam|GetDrawDebugLine
    (:then
      (bind _bblockinghit (Construct|FindMirrorPreview self))
      (if _bblockinghit
        (bind _array_element (Utilities|Array|ForEachLoopwithBreak (Variables|Beam|GetMechBeamMirrorNetwork) :!label _label)
          (:LoopBody
            (bind _success (Class|BPIMechanismBeam|CheckIsMechBeamReceiver(Message) _array_element _array_element))
            (if (not _success)
              (bind _bblockinghit_2 (Construct|FindMirrorPreview _array_element))
              (if (not _bblockinghit_2)
                (goto _label Break))
              (else
                (goto _label Break))))
          (:Completed
            (return)))
        (else
          (return))))
    (:else
      (return))))

(fn FindMirrorPreview
  (params (IsActor :type Actor%20Object%20Reference))
  (bind _beamray (Class|BPIMechanismBeam|GetMechBeamRay(Message) IsActor))
  (bind _returnvalue (Collision|BoxTraceByChannel (.Start (Utilities|Struct|BreakST_MechanismBeamRay _beamray)) (+ (.Start (Utilities|Struct|BreakST_MechanismBeamRay _beamray)) (* (.Direction (Utilities|Struct|BreakST_MechanismBeamRay _beamray)) (.BeamMaxDistance (Utilities|Struct|BreakST_MechanismBeamRay _beamray)))) (.BeamSize (Utilities|Struct|BreakST_MechanismBeamRay _beamray)) (.BeamRotation (Utilities|Struct|BreakST_MechanismBeamRay _beamray)) "TraceTypeQuery3" false (Utilities|Array|MakeArray IsActor) "ForDuration" true "(R=0.095695,G=0.000000,B=1.000000,A=1.000000)" "(R=1.000000,G=0.103386,B=0.000000,A=1.000000)" 1.0))
  (return _returnvalue))