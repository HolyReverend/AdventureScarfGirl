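; Receiver actor for a mechanical beam light puzzle that signals activation when it is identified as the beam's target.
; CheckIsMechBeamReceiver compares a given actor to itself, fires the MechBeamNetworkActivate dispatcher on a match, and returns the comparison result.
; BeginPlay binds the receiver's own handler to that dispatcher, which currently only prints a green on-screen debug message announcing puzzle activation.
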(event Custom|NetworkActivate
  (Development|PrintString "Активация головоломки со светом" true false "(R=0.000000,G=1.000000,B=0.069865,A=1.000000)"))

(event EventBeginPlay
  (|CallParentFunction)
  (EventDispatchers|BindEventtoMechBeamNetworkActivate (delegate Custom|NetworkActivate)))

(fn ConstructionScript
  (|CallParentFunction))

(fn CheckIsMechBeamReceiver
  (params (inActor :type Actor%20Object%20Reference))
  (bind _self self)
  (bind _returnvalue (== inActor _self))
  (if _returnvalue
    (Default|CallMechBeamNetworkActivate _self)
    (return _returnvalue)
    (else
      (return _returnvalue))))