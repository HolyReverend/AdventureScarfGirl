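; Base interactable door that either swings on yaw or slides left, right, up or down, as set by DoorOpeningType.
; Interact commands from the parent drive DoorTimeline, which moves MovableScene by DoorOpeningDeep and updates interaction status and direction.
; The construction script sizes collision, derives play rate from opening time, orients the arrow and poses Activated doors by rotation, even sliding types.
; CheckDoorState reports whether the door rests at its closed position.
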(event EventGetInteractTimeline
  (params (InteractTimeline :type E_InteractTimeline%20Enum :default "NewEnumerator0"))
  (|CallParentFunction InteractTimeline)
  (switch Utilities|FlowControl|Switch|SwitchonE_InteractTimeline InteractTimeline
    (:NewEnumerator0
      (bind (_direction _timeline) (Timeline|DoorTimeline Play)
        (:Update
          (Variables|Default|SetInteractDirection _direction)
          (Variables|Default|SetInteractStatus "NewEnumerator0")
          (CallFunction|DoorOpening _timeline))
        (:Finished
          (bind _output_get (Variables|Default|SetInteractDirection _direction))
          (switch Utilities|FlowControl|Switch|SwitchonETimelineDirection _output_get
            (:Forward
              (Variables|Default|SetInteractStatus "NewEnumerator1"))
            (:Backward
              (Variables|Default|SetInteractStatus "NewEnumerator2"))))))
    (:NewEnumerator1
      (Timeline|DoorTimeline PlayFromStart))
    (:NewEnumerator2
      (Timeline|DoorTimeline Stop))
    (:NewEnumerator3
      (Timeline|DoorTimeline Reverse))
    (:NewEnumerator4
      (Timeline|DoorTimeline ReverseFromEnd))))

(fn ConstructionScript
  (|CallParentFunction)
  (Components|Box|SetBoxExtent (Variables|Default|GetInteractCollision) (Variables|Default|GetInteractCollisionBox) true)
  (CallFunction|SetDoorOpeningTime)
  (switch Utilities|FlowControl|Switch|SwitchonE_DoorOpeningType (Variables|Settings|GetDoorOpeningType)
    (:NewEnumerator0
      (Transformation|SetRelativeRotation (Variables|Default|GetMovableDirectionArrow) "0.000000,90.000000,0.000000" false false)
      (switch Utilities|FlowControl|Switch|SwitchonE_InteractStatus (Variables|Default|GetInteractStatus) :!label _label
        (:NewEnumerator1
          (Transformation|SetRelativeRotation (Variables|Default|GetMovableScene) (Math|Rotator|MakeRotator 0.0 0.0 (Math|Float|SelectFloat (Variables|Settings|GetDoorOpeningDeep) 0.0 (Utilities|Enum|Equal(Enum) (Variables|Default|GetInteractStatus) "NewEnumerator1"))) false false))
        (:NewEnumerator0
          (Variables|Default|SetInteractStatus "NewEnumerator2"))))
    (:NewEnumerator1
      (Transformation|SetRelativeRotation (Variables|Default|GetMovableDirectionArrow) "0.0,180.000000,0.0" false false)
      (goto _label))
    (:NewEnumerator3
      (Transformation|SetRelativeRotation (Variables|Default|GetMovableDirectionArrow) "0, 0, 0" false false)
      (goto _label))
    (:NewEnumerator2
      (Transformation|SetRelativeRotation (Variables|Default|GetMovableDirectionArrow) "90.000000,0.000000,0.000000" false false)
      (switch Utilities|FlowControl|Switch|SwitchonE_InteractStatus (Variables|Default|GetInteractStatus) :!label _label_2
        (:NewEnumerator1
          (Transformation|SetRelativeRotation (Variables|Default|GetMovableScene) (Math|Rotator|MakeRotator 0.0 (Math|Float|SelectFloat (Variables|Settings|GetDoorOpeningDeep) 0.0 (Utilities|Enum|Equal(Enum) (Variables|Default|GetInteractStatus) "NewEnumerator1")) 0.0) false false))
        (:NewEnumerator0
          (Variables|Default|SetInteractStatus "NewEnumerator2"))))
    (:NewEnumerator4
      (Transformation|SetRelativeRotation (Variables|Default|GetMovableDirectionArrow) "-90.000000,0.000000,0.000000" false false)
      (goto _label_2))))

(fn CheckDoorState
  (bind _movablescene (Variables|Default|GetMovableScene))
  (bind _relativelocation (Variables|/Script/Engine.SceneComponent|GetRelativeLocation _movablescene))
  (bind _returnvalue (Math|Float|NearlyEqual(Float) (.z _relativelocation) 0.0 1e-06))
  (bind _returnvalue_2 (Math|Float|NearlyEqual(Float) (.x _relativelocation) 0.0 1e-06))
  (return (Utilities|Select :Index (Variables|Settings|GetDoorOpeningType) :NewEnumerator0 (Math|Float|NearlyEqual(Float) (.yaw (Variables|/Script/Engine.SceneComponent|GetRelativeRotation _movablescene)) 0.0 1e-06) :NewEnumerator1 _returnvalue_2 :NewEnumerator3 _returnvalue_2 :NewEnumerator2 _returnvalue :NewEnumerator4 _returnvalue)))

(fn SetDoorOpeningTime
  (Components|Timeline|SetPlayRate (Variables|Default|GetDoorTimeline) (/ 1.0 (Variables|Settings|GetDoorOpeningTime)))
  (return))

(fn DoorOpening
  (params (TimelineDoor :type Float%20%28double-precision%29))
  (switch Utilities|FlowControl|Switch|SwitchonE_DoorOpeningType (Variables|Settings|GetDoorOpeningType)
    (:NewEnumerator0
      (Transformation|SetRelativeRotation (Variables|Default|GetMovableScene) (Math|Rotator|MakeRotator 0.0 0.0 (* TimelineDoor (Variables|Settings|GetDoorOpeningDeep))) false false))
    (:NewEnumerator1
      (Transformation|SetRelativeLocation (Variables|Default|GetMovableScene) (Math|Vector|MakeVector (* TimelineDoor (* (Variables|Settings|GetDoorOpeningDeep) -1.0)) 0.0 0.0) false false))
    (:NewEnumerator3
      (Transformation|SetRelativeLocation (Variables|Default|GetMovableScene) (Math|Vector|MakeVector (* TimelineDoor (Variables|Settings|GetDoorOpeningDeep)) 0.0 0.0) false false))
    (:NewEnumerator2
      (Transformation|SetRelativeLocation (Variables|Default|GetMovableScene) (Math|Vector|MakeVector 0.0 0.0 (* TimelineDoor (Variables|Settings|GetDoorOpeningDeep))) false false))
    (:NewEnumerator4
      (Transformation|SetRelativeLocation (Variables|Default|GetMovableScene) (Math|Vector|MakeVector 0.0 0.0 (* TimelineDoor (* (Variables|Settings|GetDoorOpeningDeep) -1.0))) false false))))