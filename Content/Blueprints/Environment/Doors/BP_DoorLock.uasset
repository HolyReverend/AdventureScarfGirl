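; BP_DoorLock is a lockable door object that either passes interaction to its parent behavior or first demands keys from the player.
; When key locked, CheckKeys matches the player's items by name against KeyNeeds, removes the matches once all are found, and switches LockedType to Unlocked.
; It signals empty-inventory, missing-key and successful-unlock outcomes through DoorLockStatus, and ImmediatelyOpen gates whether unlocking also triggers the parent interaction.
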(event EventTick
  (params (DeltaSeconds :type Float%20%28single-precision%29))
  (|CallParentFunction DeltaSeconds))

(event EventInteracttoObject
  (switch Utilities|FlowControl|Switch|SwitchonE_InteractLockedType (Variables|LockedSettings|GetLockedType)
    (:NewEnumerator0
      (|CallParentFunction :!label _label))
    (:NewEnumerator1
      (bind _succes (CallFunction|CheckKeys))
      (if _succes
        (Variables|LockedSettings|GetImmediatelyOpen
          (:then
            (goto _label))
          (:else))))))

(event EventGetInteractTimeline
  (params (InteractTimeline :type E_InteractTimeline%20Enum :default "NewEnumerator0"))
  (|CallParentFunction InteractTimeline))

(fn ConstructionScript
  (|CallParentFunction))

(fn GetLockedType
  (return (Variables|LockedSettings|GetLockedType)))

(fn SetLockedType
  (params (InLockedType :type E_InteractLockedType%20Enum :default "NewEnumerator0"))
  (Variables|LockedSettings|SetLockedType InLockedType)
  (return true))

(fn CheckKeys
  (bind _items (Class|BPIBackpack|GetItemsfromCharacter(Message) (CallFunction|GetActualPlayer)))
  (if (Utilities|Array|IsNotEmpty _items)
    (LocalVariables|SetL_NumberNeedKeys (Utilities|Array|Length (Variables|LockedSettings|GetKeyNeeds)))
    (bind _array_element (Utilities|Array|ForEachLoopwithBreak _items :!label _label)
      (:LoopBody
        (bind _output_get (LocalVariables|SetL_FindItem _array_element))
        (if (Utilities|Array|ContainsItem (Variables|LockedSettings|GetKeyNeeds) (Utilities|Struct|BreakST_ItemDetails _output_get))
          (Utilities|Array|AddUnique (LocalVariables|GetL_FindNeedItems) (LocalVariables|GetL_FindItem))
          (bind _result (Math|Integer|DecrementInt (LocalVariables|GetL_NumberNeedKeys))
            (:%20%20
              (if (== _result 0)
                (goto _label Break))))))
      (:Completed
        (if (== (LocalVariables|GetL_NumberNeedKeys) 0)
          (bind _success (Class|BPIBackpack|RemoveItemfromCharacter(Message) (CallFunction|GetActualPlayer) (LocalVariables|GetL_FindNeedItems)))
          (if _success
            (Default|CallDoorLockStatus "NewEnumerator2")
            (bind _seccus (CallFunction|SetLockedType "NewEnumerator0"))
            (if _seccus
              (return true)
              (else
                (return false)))
            (else
              _))
          (else
            (Default|CallDoorLockStatus "NewEnumerator1")))
        (return false)))
    (else
      (Default|CallDoorLockStatus "NewEnumerator0")
      (return false))))