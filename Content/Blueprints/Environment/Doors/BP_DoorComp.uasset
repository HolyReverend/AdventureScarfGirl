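; BP_DoorComp is a door Blueprint that gates player interaction behind a lock component.
; InteracttoObject reads the lock type from BPCLocked and runs the parent interaction when Unlocked, or when Key Locked and the lock condition is true.
; The interaction behavior and construction script come from the parent class, and a debug getter exposes BPCLocked.
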(event EventInteracttoObject
  (bind _lockedtype (Default|GetLockedType (Variables|Default|GetBPC_Locked)))
  (switch Utilities|FlowControl|Switch|SwitchonE_InteractLockedType _lockedtype
    (:NewEnumerator0
      (|CallParentFunction :!label _label))
    (:NewEnumerator1
      (bind _success (Default|GetLockedCondition (Variables|Default|GetBPC_Locked)))
      (if _success
        (goto _label)))))

(fn ConstructionScript
  (|CallParentFunction))

(fn DebugGetBPC
  (return (Variables|Default|GetBPC_Locked)))