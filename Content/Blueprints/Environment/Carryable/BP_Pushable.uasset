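; BP_Pushable is an interactable environment object intended to be pushed by the interacting actor.
; Interaction toggles IsInteracted and physics simulation on PushableMesh, to which the interaction collision is attached at BeginPlay.
; Tick validates the instigator and reads its move-direction message, but the forward branch is empty.
; The interpolated movement along the mesh's forward vector is disconnected, so no push movement is applied here.
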(event EventInteracttoObject
  (Variables|Default|GetisInteracted
    (:then
      (Variables|Default|SetisInteracted false)
      (Physics|SetSimulatePhysics (Variables|Default|GetPushableMesh) false))
    (:else
      (Variables|Default|SetisInteracted true)
      (Physics|SetSimulatePhysics (Variables|Default|GetPushableMesh) true))))

(event EventBeginPlay
  (Transformation|AttachComponentToComponent (Variables|Default|GetInteractCollision) (Variables|Default|GetPushableMesh) "None" "KeepWorld" "KeepRelative" "KeepRelative" true)
  (|CallParentFunction))

(event EventTick
  (params (DeltaSeconds :type Float%20%28single-precision%29))
  (bind _instigator (CallFunction|GetInteractInstigator))
  (if (CallFunction|CheckCanIsInteract _instigator "NewEnumerator1")
    (if (Variables|Default|GetisInteracted)
      (bind _movedirection (Class|BPICharacterState|GetMoveDirection(Message) _instigator))
      (if (== (.Forward (Utilities|Struct|BreakST_CharacterMoveDirection _movedirection)) 1)
        _))))

(fn ConstructionScript
  (|CallParentFunction))