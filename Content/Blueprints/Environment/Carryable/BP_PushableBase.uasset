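; BP_PushableBase is a base Blueprint for environment objects that the player can push.
; On BeginPlay it attaches its interact collision and hint scene to the pushable mesh.
; Interacting toggles pushing through the instigator's BPC_Push component, only for the actual player, passing the object and its attach points to begin.
; The construction script adds an arrow component at each push attach point transform.
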(event Custom|PushObject
  (if (== (CallFunction|GetInteractInstigator) (CallFunction|GetActualPlayer))
    (bind _success (Class|BPIPush|GetCharacterIsPush(Message) (Actor|GetComponentbyClass (CallFunction|GetInteractInstigator) "/Game/Blueprints/Components/BPC_Push.BPC_Push_C")))
    (if (not _success)
      (Class|BPIPush|BeginInteractPush(Message) (Actor|GetComponentbyClass (CallFunction|GetInteractInstigator) "/Game/Blueprints/Components/BPC_Push.BPC_Push_C") self (Variables|Settings|GetPushAttachPoints))
      (else
        (Class|BPIPush|EndInteractPush(Message) (Actor|GetComponentbyClass (CallFunction|GetInteractInstigator) "/Game/Blueprints/Components/BPC_Push.BPC_Push_C") self)))))

(event EventInteracttoObject
  (|CallParentFunction)
  (CallFunction|PushObject))

(event EventBeginPlay
  (|CallParentFunction)
  (Transformation|AttachComponentToComponent (Variables|Default|GetInteractCollision) (Variables|Default|GetPushableMesh) "None" "KeepWorld" "KeepRelative" "KeepRelative" true)
  (Transformation|AttachComponentToComponent (Variables|Default|GetHintScene) (Variables|Default|GetPushableMesh) "None" "KeepWorld" "KeepRelative" "KeepRelative" true))

(fn ConstructionScript
  (|CallParentFunction)
  (for _array_element (Variables|Settings|GetPushAttachPoints)
    (AddComponent|AddArrowComponent false _array_element)))