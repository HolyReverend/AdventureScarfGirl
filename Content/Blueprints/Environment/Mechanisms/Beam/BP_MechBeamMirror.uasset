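; Rotatable mirror for the mech beam puzzle network, turned by interaction in fixed yaw steps.
; It starts at a negative preset yaw, with step size set so RequiredRotations turns bring it to zero.
; Interaction while deactivated starts a curve-driven RInterpTo spin on Tick, which snaps to the target when nearly reached.
; Initial placement and each completed turn broadcast a network change, to which the mirror responds by updating its beam ray.
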(event Custom|MirrorRotated
  (CallFunction|SetActualMechBeamRay))

(event EventTick
  (params (DeltaSeconds :type Float%20%28single-precision%29))
  (|CallParentFunction DeltaSeconds)
  (Variables|Default|GetIsRotated
    (:then
      (CallFunction|SpineMirror))
    (:else)))

(event EventTryInteractMechBeam
  (bind _interactablestatus (CallFunction|GetInteractStatus))
  (switch Utilities|FlowControl|Switch|SwitchonE_InteractStatus _interactablestatus
    (:NewEnumerator2
      (CallFunction|BeginRotation))))

(event EventBeginPlay
  (|CallParentFunction)
  (EventDispatchers|BindEventtoMechBeamNetworkChange (delegate Custom|MirrorRotated))
  (CallFunction|SetInitialRotationAngle))

(fn ConstructionScript
  (|CallParentFunction))

(fn BeginRotation
  (CallFunction|SetInteractStatus "NewEnumerator1")
  (Variables|Default|SetCurrentRotation (.yaw (Variables|/Script/Engine.SceneComponent|GetRelativeRotation (Variables|Default|GetMovableScene))))
  (Variables|Default|SetIsRotated true)
  (return))

(fn EndRotation
  (bind _movablescene (Variables|Default|GetMovableScene))
  (bind _relativerotation (Variables|/Script/Engine.SceneComponent|GetRelativeRotation _movablescene))
  (CallFunction|SetInteractStatus "NewEnumerator2")
  (Variables|Default|SetCurrentTime 0.0)
  (Transformation|SetRelativeRotation (Variables|Default|GetMovableScene) (Math|Rotator|MakeRotator (.roll _relativerotation) (.pitch _relativerotation) (+ (Variables|Default|GetCurrentRotation) (Variables|Default|GetDegresRotation))) true false)
  (Variables|Default|SetCurrentRotation (.yaw (Variables|/Script/Engine.SceneComponent|GetRelativeRotation (Variables|Default|GetMovableScene))))
  (Default|CallMechBeamNetworkChange)
  (Variables|Default|SetIsRotated false)
  (return))

(fn SpineMirror
  (bind _movablescene (Variables|Default|GetMovableScene))
  (bind _relativerotation (Variables|/Script/Engine.SceneComponent|GetRelativeRotation _movablescene))
  (Variables|Default|SetCurrentTime (Math|Float|Clamp(Float) (+ (Variables|Default|GetCurrentTime) (Utilities|Time|GetWorldDeltaSeconds)) 0.0 (Variables|Beam|GetAccelerationTime)))
  (Transformation|SetRelativeRotation (Variables|Default|GetMovableScene) (Math|Interpolation|RInterpTo (Variables|/Script/Engine.SceneComponent|GetRelativeRotation _movablescene) (Math|Rotator|MakeRotator (.roll _relativerotation) (.pitch _relativerotation) (Math|Rotator|NormalizeAxis (+ (Variables|Default|GetCurrentRotation) (Variables|Default|GetDegresRotation)))) (Math|Curves|GetFloatValue (Variables|Beam|GetAccelerationCurve) (/ (Variables|Default|GetCurrentTime) (Variables|Beam|GetAccelerationTime))) 1.0) true false)
  (if (Math|Float|NearlyEqual(Float) (.yaw (Variables|/Script/Engine.SceneComponent|GetRelativeRotation (Variables|Default|GetMovableScene))) (Math|Rotator|NormalizeAxis (+ (Variables|Default|GetCurrentRotation) (Variables|Default|GetDegresRotation))) 1.0)
    (CallFunction|EndRotation)
    (return)
    (else
      (return))))

(fn SetInitialRotationAngle
  (bind _movablescene (Variables|Default|GetMovableScene))
  (bind _relativerotation (Variables|/Script/Engine.SceneComponent|GetRelativeRotation _movablescene))
  (Variables|Default|SetCurrentRotation (CallFunction|AlwaysNegative(Float) (Math|Conversions|ToFloat(Integer) (Utilities|String|EnumtoString (Variables|Beam|GetInitialRotationAngle)))))
  (Transformation|SetRelativeRotation (Variables|Default|GetMovableScene) (Math|Rotator|MakeRotator (.roll _relativerotation) (.pitch _relativerotation) (Math|Rotator|NormalizeAxis (Variables|Default|GetCurrentRotation))) true false)
  (Default|CallMechBeamNetworkChange)
  (Variables|Default|SetDegresRotation (/ (Math|Float|Absolute(Float) (Variables|Default|GetCurrentRotation)) (Variables|Beam|GetRequiredRotations)))
  (return))