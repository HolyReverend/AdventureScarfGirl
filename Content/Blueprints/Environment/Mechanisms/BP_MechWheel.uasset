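; Interactable mechanism wheel that spins a movable component around yaw when its inherited interact events start or end rotation.
; Tick ramps a timer up or down through Activated, InProgress and Deactivated states, scaling speed by an acceleration curve and disabling itself once stopped.
; An optional degree limit numerically integrates that curve at BeginPlay to precompute the angle where braking starts.
; An interact-move timer is set or cleared on each start and end.
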(event EventStartInteractTimeline
  (switch Utilities|FlowControl|Switch|SwitchonE_InteractTimeline (CallFunction|GetInteractTimeline)
    (:NewEnumerator0
      (if (CallFunction|GetIsActorInsideCollision) :!label _label
        (CallFunction|BeginRotation)))
    (:NewEnumerator1
      (goto _label))
    (:NewEnumerator3
      (if (not (CallFunction|GetIsActorInsideCollision)) :!label _label_2
        (CallFunction|EndRotation)))
    (:NewEnumerator4
      (goto _label_2))))

(event EventTick
  (params (DeltaSeconds :type Float%20%28single-precision%29))
  (|CallParentFunction DeltaSeconds)
  (CallFunction|SpineWheel))

(event EventStartInteractTimelineDelay
  (CallFunction|BeginRotation))

(event EventStartInteractTimelineReturn
  (CallFunction|SwitchTimeChecker)
  (CallFunction|EndRotation))

(event EventBeginPlay
  (|CallParentFunction)
  (CallFunction|ApplyMaxDegresRotation))

(fn ConstructionScript
  (|CallParentFunction)
  (bind _interactablestatus (CallFunction|GetInteractStatus))
  (Actor|Tick|SetActorTickEnabled (Utilities|Select :Index _interactablestatus :NewEnumerator2 false :NewEnumerator1 true :NewEnumerator0 true)))

(fn SpineWheel
  (bind _movablescene (Variables|Default|GetMovableScene))
  (bind _relativerotation (Variables|/Script/Engine.SceneComponent|GetRelativeRotation _movablescene))
  (bind _interactablestatus (CallFunction|GetInteractStatus))
  (LocalVariables|SetL_InteractableStatus _interactablestatus)
  (bind _output_get (Variables|Default|SetCurrentTime (Utilities|Select :Index (LocalVariables|GetL_InteractableStatus) :NewEnumerator2 (Math|Float|Clamp(Float) (- (Variables|Default|GetCurrentTime) (Utilities|Time|GetWorldDeltaSeconds)) 0.0 (Variables|Settings|Wheel|GetAccelerationTime)) :NewEnumerator1 (Math|Float|Clamp(Float) (+ (Variables|Default|GetCurrentTime) (Utilities|Time|GetWorldDeltaSeconds)) 0.0 (Variables|Settings|Wheel|GetAccelerationTime)) :NewEnumerator0 (Variables|Settings|Wheel|GetAccelerationTime))))
  (if (not (Math|Float|NearlyEqual(Float) _output_get 0.0 1e-06))
    (if (Math|Float|NearlyEqual(Float) (Variables|Default|GetCurrentTime) (Variables|Settings|Wheel|GetAccelerationTime) 1e-06)
      (CallFunction|SetInteractStatus "NewEnumerator0"))
    (bind _output_get_2 (Variables|Default|SetWheelRotation (Math|Rotator|MakeRotator (.roll _relativerotation) (.pitch _relativerotation) (Math|Rotator|NormalizeAxis (Math|Interpolation|FInterpTo (.yaw _relativerotation) (+ (.yaw _relativerotation) (* (Variables|Settings|Wheel|GetRotationSpeed) (Math|Curves|GetFloatValue (Variables|Settings|Wheel|GetAccelerationCurve) (/ (Variables|Default|GetCurrentTime) (Variables|Settings|Wheel|GetAccelerationTime))))) (Utilities|Time|GetWorldDeltaSeconds) 1.0)))))
    (Transformation|SetRelativeRotation (Variables|Default|GetMovableScene) _output_get_2 true false)
    (Variables|Default|GetisMaxDegresRotationEnable
      (:then
        (if (Math|Float|NearlyEqual(Float) (.yaw (Variables|/Script/Engine.SceneComponent|GetRelativeRotation (Variables|Default|GetMovableScene))) (Math|Rotator|NormalizeAxis (Variables|Default|GetBrakeStartAngle)) 1.0)
          (CallFunction|SetInteractStatus "NewEnumerator2")
          (return)
          (else
            (return))))
      (:else
        (return)))
    (else
      (Actor|Tick|SetActorTickEnabled false)
      (CallFunction|FinishMovableInteract)
      (return))))

(fn DebugGetVelocity
  (return (* (Variables|Settings|Wheel|GetRotationSpeed) (/ (Variables|Default|GetCurrentTime) (Variables|Settings|Wheel|GetAccelerationTime)))))

(fn EndTemporaryRotation
  (CallFunction|SetInteractStatus "NewEnumerator2")
  (Utilities|Time|ClearandInvalidateTimerbyHandle (Variables|Default|GetInteractMoveTimeHandler))
  (return))

(fn SetTemporaryTimeRotation
  (bind _interactmovetime (CallFunction|GetInteractMoveTime))
  (if (not (Utilities|Time|IsValidTimerHandle (Variables|Default|GetInteractMoveTimeHandler)))
    (if (not (Math|Float|NearlyEqual(Float) _interactmovetime 0.0 1e-06))
      (bind _returnvalue (Utilities|Time|SetTimerbyEvent (EventDispatchers|CreateEvent :!event EndTemporaryRotation) _interactmovetime))
      (Variables|Default|SetInteractMoveTimeHandler _returnvalue)
      (return))
    (else
      (Utilities|Time|ClearandInvalidateTimerbyHandle (Variables|Default|GetInteractMoveTimeHandler))
      (return))))

(fn ApplyMaxDegresRotation
  (if (not (Math|Float|NearlyEqual(Float) (Variables|Settings|Wheel|GetMaxDegresRotation) 0.0 1e-06))
    (Variables|Default|SetisMaxDegresRotationEnable true)
    (for _index (range 0 (- (LocalVariables|GetL_Samples) 1))
      (LocalVariables|SetL_Sum (+ (Math|Curves|GetFloatValue (Variables|Settings|Wheel|GetAccelerationCurve) (/ (+ (Math|Conversions|ToFloat(Integer) _index) 0.5) (LocalVariables|GetL_Samples))) (LocalVariables|GetL_Sum))))
    (LocalVariables|SetL_Integral (/ (LocalVariables|GetL_Sum) (LocalVariables|GetL_Samples)))
    (LocalVariables|SetL_ThetaBrake (* (Variables|Settings|Wheel|GetRotationSpeed) (Variables|Settings|Wheel|GetAccelerationTime) (LocalVariables|GetL_Integral)))
    (Variables|Default|SetBrakeStartAngle (- (Variables|Settings|Wheel|GetMaxDegresRotation) (LocalVariables|GetL_ThetaBrake)))
    (return)
    (else
      (return))))

(fn BeginRotation
  (Actor|Tick|SetActorTickEnabled true)
  (CallFunction|SetInteractStatus "NewEnumerator1")
  (CallFunction|SetTemporaryTimeRotation)
  (return))

(fn EndRotation
  (CallFunction|SetInteractStatus "NewEnumerator2")
  (CallFunction|SetTemporaryTimeRotation)
  (return))