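; Base Blueprint for interactable environment objects, with a box trigger sized in the construction script and an empty InteractToObject event as the behavior hook.
; Player overlaps update the tracked actor and readiness; Overlap-type objects can fire the event directly when enabled.
; StartInteract handles explicit calls, gated by Enable/Trigger/Disable state and CheckCanIsInteract, with Trigger passing WithoutPlayer, and refuses while status is In Progress.
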(event OnComponentBeginOverlap(InteractCollision)
  (params (OverlappedComponent :type Primitive%20Component%20Object%20Reference) (OtherActor :type Actor%20Object%20Reference) (OtherComp :type Primitive%20Component%20Object%20Reference) (OtherBodyIndex :type Integer) (bFromSweep :type Boolean) (SweepResult :type Hit%20Result%20Structure%20%28by%20ref%29))
  (bind _succes (CallFunction|PlayerEnter OtherActor true))
  (if _succes
    (CallFunction|InteracttoObject)))

(event OnComponentEndOverlap(InteractCollision)
  (params (OverlappedComponent :type Primitive%20Component%20Object%20Reference) (OtherActor :type Actor%20Object%20Reference) (OtherComp :type Primitive%20Component%20Object%20Reference) (OtherBodyIndex :type Integer))
  (bind _succes (CallFunction|PlayerEnter OtherActor false))
  (if _succes
    (CallFunction|InteracttoObject)))

(event Custom|InteractToObject)

(event EventBeginPlay)

(event Collision|EventActorBeginOverlap
  (params (OtherActor :type Actor%20Object%20Reference)))

(event EventTick
  (params (DeltaSeconds :type Float%20%28single-precision%29)))

(fn ConstructionScript
  (Components|Box|SetBoxExtent (Variables|Default|GetInteractCollision) (Variables|Settings|GetInteractCollisionBox) true))

(fn PlayerEnter
  (params (InActor :type Actor%20Object%20Reference) (IsPlayerEnter :type Boolean))
  (if (CallFunction|CheckIsPlayer InActor)
    (Variables|Default|SetOverlapActor InActor)
    (if IsPlayerEnter
      (Variables|Default|GetIsPlayerInsideCollision
        (:then
          _)
        (:else
          (Variables|Default|SetIsPlayerInsideCollision IsPlayerEnter :!label _label)
          (switch Utilities|FlowControl|Switch|SwitchonE_InteractableState (Variables|Settings|GetInteractableState)
            (:NewEnumerator0
              (Variables|Default|SetIsReadyInteract IsPlayerEnter)
              (switch Utilities|FlowControl|Switch|SwitchonE_InteractType (Variables|Settings|GetInteractType)
                (:NewEnumerator0
                  (return true))
                (:NewEnumerator1
                  (return false))))
            (:NewEnumerator3
              _)
            (:NewEnumerator1
              _))
          (return false)))
      (else
        (Variables|Default|SetOverlapActor 0)
        (Variables|Default|GetIsPlayerInsideCollision
          (:then
            (goto _label))
          (:else
            _))))
    (return false)
    (else
      (return false))))

(fn GetActorInsideCollision
  (return (Variables|Default|GetOverlapActor)))

(fn GetInteractStatus
  (return (Variables|Settings|GetInteractStatus)))

(fn SetInteractableState
  (params (State :type E_InteractableState%20Enum :default "NewEnumerator0"))
  (Variables|Settings|SetInteractableState State)
  (return true))

(fn SetVisibilityInteractCollision
  (params (SetVisibility :type Boolean))
  (Development|SetHiddeninGame (Variables|Default|GetInteractCollision) (not SetVisibility) false)
  (return true))

(fn StartInteract
  (params (InActor :type Actor%20Object%20Reference))
  (switch Utilities|FlowControl|Switch|SwitchonE_InteractableState (Variables|Settings|GetInteractableState)
    (:NewEnumerator0
      (if (CallFunction|CheckCanIsInteract InActor false)
        _
        (else
          (return false))))
    (:NewEnumerator3
      (if (CallFunction|CheckCanIsInteract InActor true)
        _
        (else
          (return false))))
    (:NewEnumerator1
      (return false)))
  (switch Utilities|FlowControl|Switch|SwitchonE_InteractStatus (Variables|Settings|GetInteractStatus)
    (:NewEnumerator2
      _)
    (:NewEnumerator1
      _)
    (:NewEnumerator0
      (return false)))
  (CallFunction|InteracttoObject)
  (return true))