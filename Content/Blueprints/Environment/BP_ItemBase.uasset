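; BP_ItemBase is a base item actor that hands its data to the character on interaction and then destroys itself.
; The construction script derives the row name from an item enum, and BeginPlay loads that row from DT_Items into ItemDetails.
; StartInteract defers to the parent only for players.
; InteracttoObject sends ItemDetails to the overlapped actor by message, destroying the item only when that succeeds.
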(event EventInteracttoObject
  (bind _succes (Interaction|StartInteractwithItem (CallFunction|GetOverlappedActor)))
  (if _succes
    _))

(event EventBeginPlay
  (bind _returnvalue (Utilities|GetDataTableRow "/Game/Data/DT_Items.DT_Items" (Variables|Default|GetItemName))
    (:then
      (Variables|Default|SetItemDetails _returnvalue))))

(fn ConstructionScript
  (|CallParentFunction)
  (Variables|Default|SetItemName (Utilities|String|StringToName (Utilities|String|EnumtoString (Variables|Default|GetItemNameList)))))

(fn StartInteract
  (params (InActor :type Actor%20Object%20Reference))
  (if (CallFunction|CheckIsPlayer InActor)
    (bind _succes (|CallParentFunction InActor))
    (return _succes)
    (else
      (return false))))

(fn AfterUse
  (params (InSucces :type Boolean))
  (if InSucces
    (Actor|DestroyActor)
    (return true)
    (else
      (return false))))

(fn StartInteractwithItem
  (params (InActor :type Actor%20Object%20Reference))
  (bind _succes (Class|BPIBackpack|SendItemtoCharacter(Message) InActor (Variables|Default|GetItemDetails)))
  (bind _newparam (CallFunction|AfterUse _succes))
  (return _newparam))

(fn GetItemDetails
  (return (Variables|Default|GetItemDetails)))

(fn CheckIsItem
  (return true))