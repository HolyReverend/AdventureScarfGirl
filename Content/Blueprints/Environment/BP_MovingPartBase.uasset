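; Base Blueprint for interactable moving parts that rotate or slide a scene component by a set depth along a chosen axis.
; A timeline, rate-scaled by move time, lerps between start and target transforms, with interact status selecting forward or reverse and overlap interactions reversing mid-move.
; Optional timers delay the move or return it automatically, and end-of-move events signal completion.
; The construction script orients a direction arrow and pre-positions parts that start activated.
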(event Custom|StartInteractTimeline
  (switch Utilities|FlowControl|Switch|SwitchonE_InteractTimeline (CallFunction|GetInteractTimeline)
    (:NewEnumerator0
      (bind (_direction _timeline) (Timeline|InteractMoveTimeline Play)
        (:Update
          (Variables|Default|SetInteractDirection _direction)
          (Variables|Default|SetInteractStatus "NewEnumerator0")
          (CallFunction|InteractMoveMesh _timeline))
        (:Finished
          (bind _output_get (Variables|Default|SetInteractDirection _direction))
          (switch Utilities|FlowControl|Switch|SwitchonETimelineDirection _output_get
            (:Forward
              (Variables|Default|SetInteractStatus "NewEnumerator1"))
            (:Backward
              (Variables|Default|SetInteractStatus "NewEnumerator2")))
          (CallFunction|FinishMovableInteract))))
    (:NewEnumerator1
      (Timeline|InteractMoveTimeline PlayFromStart))
    (:NewEnumerator2
      (Timeline|InteractMoveTimeline Stop))
    (:NewEnumerator3
      (Timeline|InteractMoveTimeline Reverse))
    (:NewEnumerator4
      (Timeline|InteractMoveTimeline ReverseFromEnd))))

(event Custom|StartInteractTimelineDelay
  (switch Utilities|FlowControl|Switch|SwitchonE_InteractTimeline (CallFunction|GetInteractTimeline)
    (:NewEnumerator0
      (bind (_direction _timeline) (Timeline|InteractMoveTimeline Play)
        (:Update
          (Variables|Default|SetInteractDirection _direction)
          (Variables|Default|SetInteractStatus "NewEnumerator0")
          (CallFunction|InteractMoveMesh _timeline))
        (:Finished
          (bind _output_get (Variables|Default|SetInteractDirection _direction))
          (switch Utilities|FlowControl|Switch|SwitchonETimelineDirection _output_get
            (:Forward
              (Variables|Default|SetInteractStatus "NewEnumerator1"))
            (:Backward
              (Variables|Default|SetInteractStatus "NewEnumerator2")))
          (CallFunction|FinishMovableInteract))))
    (:NewEnumerator1
      (Timeline|InteractMoveTimeline PlayFromStart))
    (:NewEnumerator2
      (Timeline|InteractMoveTimeline Stop))
    (:NewEnumerator3
      (Timeline|InteractMoveTimeline Reverse))
    (:NewEnumerator4
      (Timeline|InteractMoveTimeline ReverseFromEnd))))

(event Custom|StartInteractTimelineReturn
  (Timers|SwitchTimeChecker)
  (switch Utilities|FlowControl|Switch|SwitchonE_InteractTimeline (CallFunction|GetInteractTimeline)
    (:NewEnumerator0
      (bind (_direction _timeline) (Timeline|InteractMoveTimeline Play)
        (:Update
          (Variables|Default|SetInteractDirection _direction)
          (Variables|Default|SetInteractStatus "NewEnumerator0")
          (CallFunction|InteractMoveMesh _timeline))
        (:Finished
          (bind _output_get (Variables|Default|SetInteractDirection _direction))
          (switch Utilities|FlowControl|Switch|SwitchonETimelineDirection _output_get
            (:Forward
              (Variables|Default|SetInteractStatus "NewEnumerator1"))
            (:Backward
              (Variables|Default|SetInteractStatus "NewEnumerator2")))
          (CallFunction|FinishMovableInteract))))
    (:NewEnumerator1
      (Timeline|InteractMoveTimeline PlayFromStart))
    (:NewEnumerator2
      (Timeline|InteractMoveTimeline Stop))
    (:NewEnumerator3
      (Timeline|InteractMoveTimeline Reverse))
    (:NewEnumerator4
      (Timeline|InteractMoveTimeline ReverseFromEnd))))

(event EventBeginPlay
  (Variables|Default|SetTargetSceneRTransform (CallFunction|GetTargetSceneTransform false))
  (|CallParentFunction))

(event EventInteracttoObject
  (if (not (Utilities|Time|IsValidTimerHandle (Variables|Default|GetReturnTimeHandler)))
    (|CallParentFunction)
    (bind _succes (Timers|SetDelayInteract))
    (bind _succes_2 (Timers|SetReturnTime))
    (if (not _succes)
      (if (or (not _succes_2) (not (Utilities|Time|IsValidTimerHandle (Variables|Default|GetDelayInteractHandler))))
        (CallFunction|StartInteractTimeline)))))

(event EventTick
  (params (DeltaSeconds :type Float%20%28single-precision%29))
  (|CallParentFunction DeltaSeconds))

(fn ConstructionScript
  (|CallParentFunction)
  (Variables|Default|SetStartSceneRTransform (Transformation|GetRelativeTransform (Variables|Default|GetMovableScene)))
  (Construction|SetPlayRateTimeline)
  (Debug|SetDirectionArrow)
  (Construction|SetInteractTypePosition))

(fn GetInteractTimeline
  (switch Utilities|FlowControl|Switch|SwitchonE_InteractStatus (Variables|Default|GetInteractStatus)
    (:NewEnumerator2
      (bind _output_get (Variables|Default|SetInteractTimeline "NewEnumerator1")))
    (:NewEnumerator1
      (bind _output_get_2 (Variables|Default|SetInteractTimeline "NewEnumerator4")))
    (:NewEnumerator0
      (switch Utilities|FlowControl|Switch|SwitchonE_InteractType (Variables|Default|GetInteractType)
        (:NewEnumerator0
          (switch Utilities|FlowControl|Switch|SwitchonETimelineDirection (Variables|Default|GetInteractDirection)
            (:Forward
              (bind _output_get_3 (Variables|Default|SetInteractTimeline "NewEnumerator3")))
            (:Backward
              (bind _output_get_4 (Variables|Default|SetInteractTimeline "NewEnumerator0")))))
        (:NewEnumerator1
          (return "NewEnumerator5")))))
  (return (Utilities|Select :Index (Variables|Default|GetInteractTimeline) :NewEnumerator0 _output_get_4 :NewEnumerator1 _output_get :NewEnumerator2 "NewEnumerator2" :NewEnumerator3 _output_get_3 :NewEnumerator4 _output_get_2 :NewEnumerator5 "NewEnumerator5")))

(fn InteractMoveMesh
  (params (TimelineMoving :type Float%20%28double-precision%29))
  (Transformation|SetRelativeTransform (Variables|Default|GetMovableScene) (Math|Transform|Lerp(Transform) (Variables|Default|GetStartSceneRTransform) (Variables|Default|GetTargetSceneRTransform) TimelineMoving) false false)
  (return))

(fn SetPlayRateTimeline
  (Components|Timeline|SetPlayRate (Variables|Default|GetInteractMoveTimeline) (/ 1.0 (Variables|Settings|Timers|GetInteractMoveTime)))
  (return))

(fn SetDirectionArrow
  (bind _displacementdepth_ (Variables|Settings|General|GetDisplacementDepth%20))
  (bind _returnvalue (> _displacementdepth_ 0.0))
  (bind _returnvalue_2 (Math|Float|SelectFloat 1.0 -1.0 _returnvalue))
  (bind _returnvalue_3 (* 9e+01 _returnvalue_2))
  (Transformation|SetRelativeRotation (Variables|Default|GetMovableDirectionArrow) (Utilities|Select :Index (Variables|Settings|Type|GetInteractMovingType) :NewEnumerator0 (Math|Rotator|MakeRotator 0.0 0.0 (* 135.0 _returnvalue_2)) :NewEnumerator6 (Math|Rotator|MakeRotator 0.0 -45.0 _returnvalue_3) :NewEnumerator7 (Math|Rotator|MakeRotator 0.0 (* 1.8e+02 (Math|Float|SelectFloat 0.0 1.0 _returnvalue)) 0.0) :NewEnumerator1 (Math|Rotator|MakeRotator 0.0 0.0 _returnvalue_3) :NewEnumerator3 (Math|Rotator|MakeRotator 0.0 _returnvalue_3 0.0)) false false)
  (return))

(fn GetValueInteractStatus
  (params (InValue :type Float%20%28double-precision%29) (IsConstruct :type Boolean))
  (return (Math|Float|SelectFloat (+ (Variables|Settings|General|GetDisplacementDepth%20) InValue) (Math|Float|SelectFloat InValue (+ InValue (Variables|Settings|General|GetDisplacementDepth%20)) IsConstruct) (Utilities|Enum|Equal(Enum) (Variables|Default|GetInteractStatus) "NewEnumerator1"))))

(fn SetInteractTypePosition
  (switch Utilities|FlowControl|Switch|SwitchonE_InteractStatus (Variables|Default|GetInteractStatus)
    (:NewEnumerator2
      _)
    (:NewEnumerator1
      (Transformation|SetRelativeTransform (Variables|Default|GetMovableScene) (CallFunction|GetTargetSceneTransform true) false false)
      (return))
    (:NewEnumerator0
      (Variables|Default|SetInteractStatus "NewEnumerator2")))
  (return))

(fn ClearDelayInteractHandler
  (Utilities|Time|ClearandInvalidateTimerbyHandle (Variables|Default|GetDelayInteractHandler))
  (return))

(fn GetDelayInteractHandlerValidate
  (return (Utilities|Time|IsValidTimerHandle (Variables|Default|GetDelayInteractHandler))))

(fn SetReturnTime
  (if (not (Math|Float|NearlyEqual(Float) (Variables|Settings|Timers|GetReturnTime) 0.0 1e-06))
    (if (not (Utilities|Time|IsValidTimerHandle (Variables|Default|GetReturnTimeHandler)))
      (bind _returnvalue (Utilities|Time|SetTimerbyEvent (EventDispatchers|CreateEvent :!event Custom|StartInteractTimelineReturn) (+ (Variables|Settings|Timers|GetDelayInteract) (Variables|Settings|Timers|GetReturnTime))))
      (Variables|Default|SetReturnTimeHandler _returnvalue)
      (return true)
      (else
        (Timers|ClearReturnTimeHandler)
        (return true)))
    (else
      (return false))))

(fn ClearReturnTimeHandler
  (Utilities|Time|ClearandInvalidateTimerbyHandle (Variables|Default|GetReturnTimeHandler))
  (return))

(fn SetDelayInteract
  (if (not (Math|Float|NearlyEqual(Float) (Variables|Settings|Timers|GetDelayInteract) 0.0 1e-06))
    (bind _isvalidate (CallFunction|GetDelayInteractHandlerValidate))
    (if (not _isvalidate)
      (bind _returnvalue (Utilities|Time|SetTimerbyEvent (EventDispatchers|CreateEvent :!event Custom|StartInteractTimelineDelay) (Variables|Settings|Timers|GetDelayInteract)))
      (Variables|Default|SetDelayInteractHandler _returnvalue)
      (EventDispatchers|BindEventtoEndMoveInteract (EventDispatchers|CreateEvent :!event ClearDelayInteractHandler))
      (return true)
      (else
        (Timers|ClearDelayInteractHandler)
        (return true)))
    (else
      (return false))))

(fn GetReturnInteractHandlerValidate
  (return (Utilities|Time|IsValidTimerHandle (Variables|Default|GetReturnTimeHandler))))

(fn GetReturnTimeValid
  (return (not (Math|Float|NearlyEqual(Float) (Variables|Settings|Timers|GetReturnTime) 0.0 1e-06))))

(fn GetReturnTotalDelayTime
  (return (+ (Variables|Settings|Timers|GetDelayInteract) (Variables|Settings|Timers|GetReturnTime))))

(fn GetTargetSceneTransform
  (params (IsConstruct :type Boolean))
  (bind _startscenertransform (Variables|Default|GetStartSceneRTransform))
  (bind _startscenertransform_2 (Variables|Default|GetStartSceneRTransform))
  (bind _startscenertransform_3 (Variables|Default|GetStartSceneRTransform))
  (bind _startscenertransform_4 (Variables|Default|GetStartSceneRTransform))
  (bind _startscenertransform_5 (Variables|Default|GetStartSceneRTransform))
  (bind (_roll _pitch _yaw) (Math|Rotator|BreakRotator (.rotation _startscenertransform_3)))
  (bind (_roll_2 _pitch_2 _yaw_2) (Math|Rotator|BreakRotator (.rotation _startscenertransform_2)))
  (bind (_x _y _z) (Math|Vector|BreakVector (.location _startscenertransform)))
  (bind (_x_2 _y_2 _z_2) (Math|Vector|BreakVector (.location _startscenertransform_4)))
  (bind (_x_3 _y_3 _z_3) (Math|Vector|BreakVector (.location _startscenertransform_5)))
  (return (Utilities|Select :Index (Variables|Settings|Type|GetInteractMovingType) :NewEnumerator0 (Math|Transform|MakeTransform (.location _startscenertransform_2) (Math|Rotator|MakeRotator _roll_2 _pitch_2 (Construction|GetValueInteractStatus _yaw_2 IsConstruct)) (.scale _startscenertransform_2)) :NewEnumerator6 (Math|Transform|MakeTransform (.location _startscenertransform_3) (Math|Rotator|MakeRotator (Construction|GetValueInteractStatus _roll IsConstruct) _pitch _yaw) (.scale _startscenertransform_3)) :NewEnumerator7 (Math|Transform|MakeTransform (Math|Vector|MakeVector (Construction|GetValueInteractStatus _x_2 IsConstruct) _y_2 _z_2) (.rotation _startscenertransform_4) (.scale _startscenertransform_4)) :NewEnumerator1 (Math|Transform|MakeTransform (Math|Vector|MakeVector _x_3 (Construction|GetValueInteractStatus _y_3 IsConstruct) _z_3) (.rotation _startscenertransform_5) (.scale _startscenertransform_5)) :NewEnumerator3 (Math|Transform|MakeTransform (Math|Vector|MakeVector _x _y (Construction|GetValueInteractStatus _z IsConstruct)) (.rotation _startscenertransform) (.scale _startscenertransform)))))

(fn FinishMovableInteract
  (Default|CallEndMoveInteract)
  (if (Utilities|Time|IsValidTimerHandle (Variables|Default|GetReturnTimeHandler))
    (Variables|Default|GetReturnTimeChecker
      (:then
        (Timers|ClearReturnTimeHandler)
        (Variables|Default|SetReturnTimeChecker false)
        (Default|CallCompleteInteract)
        (return))
      (:else))
    (else
      (return))))

(fn SwitchTimeChecker
  (Variables|Default|SetReturnTimeChecker (not (Variables|Default|GetReturnTimeChecker)))
  (return))

(fn GetInteractMoveTime
  (return (Variables|Settings|Timers|GetInteractMoveTime)))

(fn SetInteractMoveTime
  (params (InInteractMoveTime :type Float%20%28double-precision%29))
  (Variables|Settings|Timers|SetInteractMoveTime InInteractMoveTime)
  (return))