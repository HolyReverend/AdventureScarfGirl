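; BP_PlayerCharacter is the player character, holding an item inventory and taking part in game save and load.
; Item functions to send, get and remove delegate to the BPCBackpack component, and a getter exposes the camera's world transform.
; Interface-driven SaveData packs actor transform, control rotation and backpack items into the save's PlayerData.
; LoadData applies them back, then resets speed and jump.
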(fn ConstructionScript
  (|CallParentFunction))

(fn GetPlayerCameraTransform
  (return (Transformation|GetWorldTransform (Variables|Camera|GetCamera))))

(fn GetItemsfromCharacter
  (return (Default|GetItemsfromBackpack (Variables|Default|GetBPC_Backpack))))

(fn LoadData
  (params (InLoadData :type BP%20Save%20Game%20Object%20Reference))
  ;[0.15 0.15 0.15 0.5] При активации Загрузки игры - по имплементированному интерфейсу получаем данные из SaveData, необходимые применить в текущем Акторе.
  (Transformation|SetActorTransform (Utilities|Struct|BreakST_SaveLoadData (Variables|/Game/SaveGame/BP_SaveGame.BP_SaveGame_C|GetPlayerData InLoadData)))
  (Pawn|SetControlRotation (Game|GetPlayerController 0) (Utilities|Struct|BreakST_SaveLoadData (Variables|/Game/SaveGame/BP_SaveGame.BP_SaveGame_C|GetPlayerData InLoadData)))
  (Default|SetItemstoBackpack (Variables|Default|GetBPC_Backpack) (Utilities|Struct|BreakST_SaveLoadData (Variables|/Game/SaveGame/BP_SaveGame.BP_SaveGame_C|GetPlayerData InLoadData)))
  (bind _success (CallFunction|ResetSpeedandJump true))
  (return _success))

(fn RemoveItemfromCharacter
  (params (InItem :type Array%20of%20ST%20Item%20Details%20Structures))
  (bind _success (Default|RemoveItemfromBackpack (Variables|Default|GetBPC_Backpack) InItem))
  (return _success))

(fn SaveData
  (params (InSaveData :type BP%20Save%20Game%20Object%20Reference))
  ;[0.15 0.15 0.15 0.5] При активации Сохранения игры - по имплементированному интерфейсу сохраняем данные в SaveData.
  (Variables|/Game/SaveGame/BP_SaveGame.BP_SaveGame_C|SetPlayerData InSaveData (Utilities|Struct|MakeST_SaveLoadData (Transformation|GetActorTransform) (Pawn|GetControlRotation (Game|GetPlayerController 0) :!class /Script/Engine.Controller) (Default|GetItemsfromBackpack (Variables|Default|GetBPC_Backpack))))
  (return true))

(fn SendItemtoCharacter
  (params (InItemDetails :type ST%20Item%20Details%20Structure))
  (Default|SetItemtoBackpack (Variables|Default|GetBPC_Backpack) InItemDetails)
  (return true))