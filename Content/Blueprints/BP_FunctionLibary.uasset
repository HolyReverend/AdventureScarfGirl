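; Blueprint function library of shared gameplay, debug and math helpers.
; Player helpers treat the pawn controlled by player controller 0 as the player, and an interaction check filters actors by target type: player, BPI_Interactable implementers, or either.
; Other utilities print an on-screen separator, copy text render component settings with optional relative transform, and force float or integer values to non-positive via negated absolute value.
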(fn CheckIsPlayer
  (params (InActor :type Actor%20Object%20Reference))
  (return (== InActor (Pawn|GetControlledPawn (Game|GetPlayerController 0)))))

(fn PrintSeparator
  (params (InTimeDuration :type Float%20%28single-precision%29) (InKey :type Name))
  (Development|PrintText 0 (Utilities|Text|FormatText "--------------------------------") true false "(R=0.896269,G=0.032944,B=0.000000,A=1.000000)" InTimeDuration InKey)
  (return))

(fn CheckCanIsInteract
  (params (InActor :type Actor%20Object%20Reference) (TargetActorType :type E_InteractTargetActorType%20Enum :default "NewEnumerator0"))
  (switch Utilities|FlowControl|Switch|SwitchonE_InteractTargetActorType TargetActorType
    (:NewEnumerator0
      (return (or (Checker|CheckIsPlayer InActor) (Utilities|DoesObjectImplementInterface InActor "/Game/Blueprints/Interfaces/Interactable/BPI_Interactable.BPI_Interactable_C"))))
    (:NewEnumerator1
      (return (Checker|CheckIsPlayer InActor)))
    (:NewEnumerator2
      (return (Utilities|DoesObjectImplementInterface InActor "/Game/Blueprints/Interfaces/Interactable/BPI_Interactable.BPI_Interactable_C")))))

(fn GetActualPlayer
  (return (Pawn|GetControlledPawn (Game|GetPlayerController 0))))

(fn CopyTextRenderSettings
  (params (SourceComponent :type BPC%20Hint%20Key%20Text%20Object%20Reference) (TargetComponent :type BPC%20Hint%20Key%20Text%20Object%20Reference%20%28by%20ref%29) (isCopyTransform :type Boolean))
  (Class|TextRenderComponent|SetFont TargetComponent (Variables|/Script/Engine.TextRenderComponent|GetFont SourceComponent))
  (Rendering|Components|TextRender|SetText TargetComponent (Variables|/Script/Engine.TextRenderComponent|GetText SourceComponent))
  (Rendering|Components|TextRender|SetWorldSize TargetComponent (Variables|/Script/Engine.TextRenderComponent|GetWorldSize SourceComponent))
  (Rendering|Components|TextRender|SetTextRenderColor TargetComponent (Variables|/Script/Engine.TextRenderComponent|GetTextRenderColor SourceComponent))
  (Rendering|Components|TextRender|SetHorizontalAlignment TargetComponent (Variables|/Script/Engine.TextRenderComponent|GetHorizontalAlignment SourceComponent))
  (Class|TextRenderComponent|SetVerticalAlignment TargetComponent (Variables|/Script/Engine.TextRenderComponent|GetVerticalAlignment SourceComponent))
  (Rendering|SetVisibility TargetComponent (Variables|/Script/Engine.SceneComponent|GetbVisible SourceComponent) false)
  (Development|SetHiddeninGame TargetComponent (Variables|/Script/Engine.SceneComponent|GetbHiddenInGame SourceComponent) false)
  (Class|TextRenderComponent|SetTextMaterial TargetComponent (Variables|/Script/Engine.TextRenderComponent|GetTextMaterial SourceComponent))
  (if isCopyTransform
    (Transformation|SetRelativeTransform TargetComponent (Transformation|GetRelativeTransform SourceComponent) false false)
    (return)
    (else
      (return))))

(fn AlwaysNegative(Float)
  (params (InValue :type Float%20%28double-precision%29))
  (return (* (Math|Float|Absolute(Float) InValue) -1.0)))

(fn AlwaysNegative(Integer)
  (params (InValue :type Integer))
  (return (* (Math|Integer|Absolute(Integer) InValue) -1)))