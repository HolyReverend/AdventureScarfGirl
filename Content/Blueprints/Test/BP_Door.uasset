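; BP_Door is a sliding door actor that opens when something overlaps its trigger and can auto-close after a delay.
; Overlap events drive open and close requests, with timer handles for the optional open delay and auto-close.
; An Opening/Open/Closing/Closed state enum guards a single timeline, played or reversed to lerp the mesh to an offset.
; Only a Side (X) offset is wired, and end overlap zeroes the count instead of decrementing it.
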(event OnComponentBeginOverlap(Trigger)
  (params (OverlappedComponent :type Primitive%20Component%20Object%20Reference) (OtherActor :type Actor%20Object%20Reference) (OtherComp :type Primitive%20Component%20Object%20Reference) (OtherBodyIndex :type Integer) (bFromSweep :type Boolean) (SweepResult :type Hit%20Result%20Structure%20%28by%20ref%29))
  (Math|Integer|IncrementInt (Variables|Default|GetOverlapCount%20)
    (:%20%20
      (CallFunction|OpenRequest))))

(event OnComponentEndOverlap(Trigger)
  (params (OverlappedComponent :type Primitive%20Component%20Object%20Reference) (OtherActor :type Actor%20Object%20Reference) (OtherComp :type Primitive%20Component%20Object%20Reference) (OtherBodyIndex :type Integer))
  (Variables|Default|SetOverlapCount%20 0)
  (if (and (== (Variables|Default|GetOverlapCount%20) 0) (Utilities|Enum|Equal(Enum) (Variables|Default|GetEDoorState) "NewEnumerator2"))
    (if (Variables|Default|GetAutoClose)
      (bind _returnvalue (Utilities|Time|SetTimerbyEvent (EventDispatchers|CreateEvent :!event Custom|CloseRequest) (Variables|Default|GetAutoCloseDelay)))
      (Variables|Default|SetTH_AutoClose _returnvalue)
      (else
        (CallFunction|CloseRequest)))))

(event Custom|CloseRequest
  (Variables|Default|SetbDesiredOpen%20 false)
  (Utilities|Time|ClearandInvalidateTimerbyHandle (Variables|Default|GetTH_OpenDelay))
  (if (== (Variables|Default|GetOverlapCount%20) 0)
    (CallFunction|StartClosing)))

(event Custom|OpenRequest
  (Variables|Default|SetbDesiredOpen%20 true)
  (Utilities|Time|ClearandInvalidateTimerbyHandle (Variables|Default|GetTH_OpenDelay))
  (Utilities|Time|ClearandInvalidateTimerbyHandle (Variables|Default|GetTH_AutoClose))
  (if (> (Variables|Default|GetOpenDelay) 0.0)
    (bind _returnvalue (Utilities|Time|SetTimerbyEvent (EventDispatchers|CreateEvent :!event Custom|StartOpenening) (Variables|Default|GetOpenDelay)))
    (Variables|Default|SetTH_OpenDelay _returnvalue)
    (else
      (CallFunction|StartOpenening))))

(event Custom|StartClosing
  (if (not (or (Utilities|Enum|Equal(Enum) (Variables|Default|GetEDoorState) "NewEnumerator3") (Utilities|Enum|Equal(Enum) (Variables|Default|GetEDoorState) "NewEnumerator0")))
    (if (not (> (Variables|Default|GetOverlapCount%20) 0))
      (Variables|Default|SetEDoorState "NewEnumerator3")
      (bind _alpha (Timeline|TL_Open Reverse)
        (:Update
          (Transformation|SetRelativeLocation (Variables|Default|GetDoorMesh%20) (Math|Vector|Lerp(Vector) (Variables|Default|GetStartLoc) (Variables|Default|GetTargetLoc) _alpha) false false))
        (:Finished
          (switch Utilities|FlowControl|Switch|SwitchonEDoorState (Variables|Default|GetEDoorState)
            (:NewEnumerator0
              (if (and (Variables|Default|GetAutoClose) (== (Variables|Default|GetOverlapCount%20) 0)) :!label _label
                (Utilities|Time|ClearandInvalidateTimerbyHandle (Variables|Default|GetTH_AutoClose))
                (bind _returnvalue (Utilities|Time|SetTimerbyEvent (EventDispatchers|CreateEvent :!event Custom|CloseRequest) (Variables|Default|GetAutoCloseDelay)))
                (Variables|Default|SetTH_AutoClose _returnvalue)
                (else
                  (Variables|Default|SetEDoorState "NewEnumerator0"))))
            (:NewEnumerator2
              (Variables|Default|SetEDoorState "NewEnumerator2" :!label _label_2))
            (:NewEnumerator1
              (goto _label_2))
            (:NewEnumerator3
              (goto _label))))))))

(event Custom|StartOpenening
  (if (not (or (Utilities|Enum|Equal(Enum) (Variables|Default|GetEDoorState) "NewEnumerator1") (Utilities|Enum|Equal(Enum) (Variables|Default|GetEDoorState) "NewEnumerator2")))
    (Utilities|Time|ClearandInvalidateTimerbyHandle (Variables|Default|GetTH_AutoClose))
    (Variables|Default|SetEDoorState "NewEnumerator1")
    (bind _alpha (Timeline|TL_Open Play)
      (:Update
        (Transformation|SetRelativeLocation (Variables|Default|GetDoorMesh%20) (Math|Vector|Lerp(Vector) (Variables|Default|GetStartLoc) (Variables|Default|GetTargetLoc) _alpha) false false))
      (:Finished
        (switch Utilities|FlowControl|Switch|SwitchonEDoorState (Variables|Default|GetEDoorState)
          (:NewEnumerator0
            (if (and (Variables|Default|GetAutoClose) (== (Variables|Default|GetOverlapCount%20) 0)) :!label _label
              (Utilities|Time|ClearandInvalidateTimerbyHandle (Variables|Default|GetTH_AutoClose))
              (bind _returnvalue (Utilities|Time|SetTimerbyEvent (EventDispatchers|CreateEvent :!event Custom|CloseRequest) (Variables|Default|GetAutoCloseDelay)))
              (Variables|Default|SetTH_AutoClose _returnvalue)
              (else
                (Variables|Default|SetEDoorState "NewEnumerator0"))))
          (:NewEnumerator2
            (Variables|Default|SetEDoorState "NewEnumerator2" :!label _label_2))
          (:NewEnumerator1
            (goto _label_2))
          (:NewEnumerator3
            (goto _label)))))))

(event EventBeginPlay
  (Variables|Default|SetStartLoc (Variables|/Script/Engine.SceneComponent|GetRelativeLocation (Variables|Default|GetDoorMesh%20)))
  (switch Utilities|FlowControl|Switch|SwitchonEDoorOffsetType (Variables|Default|GetEDoorOffsetType)
    (:NewEnumerator0
      (Variables|Default|SetTargetLoc (Math|Vector|MakeVector (+ (Variables|Default|GetOffsetDistance%20) (.x (Variables|Default|GetStartLoc))) (.y (Variables|Default|GetStartLoc)) (.z (Variables|Default|GetStartLoc)))))))

(event Collision|EventActorBeginOverlap
  (params (OtherActor :type Actor%20Object%20Reference)))

(event EventTick
  (params (DeltaSeconds :type Float%20%28single-precision%29)))

(fn ConstructionScript)